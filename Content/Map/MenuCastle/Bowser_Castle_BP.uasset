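; Bowser's castle actor for the menu map, which animates and sounds its main and back doors opening.
; A custom OpenDoorEvent plays the main door animation with the opening sound.
; Tick polls MarioGameInstance for the main menu Play press, then a DoOnce opens the back door once with the same animation and sound at a reduced play rate.
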(event Custom|OpenDoorEvent
  (Components|Animation|PlayAnimation (Variables|Default|GetMain_Door) "/Game/Map/MenuCastle/Castle_Door_Animation.Castle_Door_Animation" false)
  (Audio|PlaySound2D "/Game/Sound_Effects/Castle_Door_Opening.Castle_Door_Opening" 1.0 1.0 0.0 0 0))

(event EventTick
  (params (DeltaSeconds :type Float%20%28single-precision%29))
  (bind _back_door (Variables|Default|GetBack_Door))
  (bind _asmario_game_instance (Utilities|Casting|CastToMarioGameInstance (Game|GetGameInstance)))
  (if (Variables|/Game/MarioGameInstance.MarioGameInstance_C|GetMainMenuPlayIsPressed _asmario_game_instance)
    (Utilities|FlowControl|DoOnce false
      (:Completed
        (Components|Animation|PlayAnimation _back_door "/Game/Map/MenuCastle/Castle_Door_Animation.Castle_Door_Animation" false)
        (Components|Timeline|SetPlayRate _back_door 0.7)
        (Audio|PlaySound2D "/Game/Sound_Effects/Castle_Door_Opening.Castle_Door_Opening" 1.0 1.0 0.0 0 0)))))

(fn ConstructionScript)