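; Exit pipe for dungeons and transition levels that plays Mario's pipe animation and loads the next level.
; When a walking Mario overlaps the capsule, it disables movement, input and top collision, then plays the pipe sound.
; GameInstance progress flags select the Level Sequence and destination: Main, Level2 or Level2Finish.
; Mario is hidden during the cinematic, flags update in most branches, and fixed delays time the level load.
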(event OnComponentBeginOverlap(Capsule)
  (params (OverlappedComponent :type Primitive%20Component%20Object%20Reference) (OtherActor :type Actor%20Object%20Reference) (OtherComp :type Primitive%20Component%20Object%20Reference) (OtherBodyIndex :type Integer) (bFromSweep :type Boolean) (SweepResult :type Hit%20Result%20Structure%20%28by%20ref%29))
  ;[1 1 1] Desired animations for when exiting pipe
  (bind _asmario_bp (Utilities|Casting|CastToMario_BP OtherActor))
  (bind _output_get (Variables|Default|SetMario _asmario_bp))
  (if (Pawn|Components|CharacterMovement|IsWalking (Variables|/Script/Engine.Character|GetCharacterMovement _output_get))
    (bind _asmario_game_instance (Utilities|Casting|CastToMarioGameInstance (Game|GetGameInstance)))
    (Variables|Default|SetAs%20Mario%20Game%20Instance _asmario_game_instance)
    (Transformation|SetActorRotation (Variables|Default|GetMario))
    (Pawn|Components|CharacterMovement|DisableMovement (Variables|/Script/Engine.Character|GetCharacterMovement _output_get))
    (Input|DisableInput (Game|GetPlayerCharacter 0) 0)
    (Default|ExitPipeAnimation (Variables|Default|GetMario))
    (Utilities|FlowControl|Delay 0.1)
    (Collision|SetCollisionEnabled (Variables|Default|GetTopCollision) "NoCollision")
    (Utilities|FlowControl|Delay 0.4)
    (Audio|PlaySound2D "/Game/Sound_Effects/PipeEnterExit.PipeEnterExit" 1.0 1.0 0.0 0 0)
    ;[1 1 1] Checking in which level mario is / playing desired animations and opening correct levels
    (if (Variables|/Game/MarioGameInstance.MarioGameInstance_C|GetEnteredTransitionLevel (Variables|Default|GetAs%20Mario%20Game%20Instance))
      (if (Variables|/Game/MarioGameInstance.MarioGameInstance_C|GetExitLevel2 (Variables|Default|GetAs%20Mario%20Game%20Instance))
        ;[1 1 1] If mario has entered the transition level and has exited level 2
        (bind _outactor (Sequencer|Player|CreateLevelSequencePlayer "/Game/Sequences/Level_2/ExitLevel2Sequence.ExitLevel2Sequence"))
        (Sequencer|Player|Play (Variables|/Script/LevelSequence.LevelSequenceActor|GetSequencePlayer _outactor) :!class /Script/MovieScene.MovieSceneSequencePlayer)
        (Rendering|SetActorHiddenInGame (Variables|Default|GetMario) true)
        (Utilities|FlowControl|Delay 2.05)
        (Game|OpenLevel(byName) "Level2Finish" false)
        (else
          ;[1 1 1] Mario has entered transition level and has entered level 2 so playing pipe desired animations
          (if (Variables|/Game/MarioGameInstance.MarioGameInstance_C|GetEnteredLevel2 (Variables|Default|GetAs%20Mario%20Game%20Instance))
            (Variables|/Game/MarioGameInstance.MarioGameInstance_C|SetEnteredLevel2Pipe (Variables|Default|GetAs%20Mario%20Game%20Instance) false)
            (Variables|/Game/MarioGameInstance.MarioGameInstance_C|SetExitLevel2Pipe (Variables|Default|GetAs%20Mario%20Game%20Instance) true)
            (bind _outactor_2 (Sequencer|Player|CreateLevelSequencePlayer "/Game/Sequences/ExitDungeonSequencee.ExitDungeonSequencee"))
            (Sequencer|Player|Play (Variables|/Script/LevelSequence.LevelSequenceActor|GetSequencePlayer _outactor_2) :!class /Script/MovieScene.MovieSceneSequencePlayer)
            (Rendering|SetActorHiddenInGame (Variables|Default|GetMario) true)
            (Utilities|FlowControl|Delay 2.05)
            (Game|OpenLevel(byName) "Level2" false)
            (else
              ;[1 1 1] Mario has entered transition level and hasn't entered level 2 yet
              (bind _outactor_3 (Sequencer|Player|CreateLevelSequencePlayer "/Game/Sequences/TransitionLevel/EnterLevel2FromTransitionSequence.EnterLevel2FromTransitionSequence"))
              (Sequencer|Player|Play (Variables|/Script/LevelSequence.LevelSequenceActor|GetSequencePlayer _outactor_3) :!class /Script/MovieScene.MovieSceneSequencePlayer)
              (Rendering|SetActorHiddenInGame (Variables|Default|GetMario) true)
              (Utilities|FlowControl|Delay 2.05)
              (Variables|/Game/MarioGameInstance.MarioGameInstance_C|SetExitTransitionLevel (Variables|Default|GetAs%20Mario%20Game%20Instance) true)
              (Variables|/Game/MarioGameInstance.MarioGameInstance_C|SetEnteredLevel2 (Variables|Default|GetAs%20Mario%20Game%20Instance) true)
              (Game|OpenLevel(byName) "Level2" false)))))
      (else
        ;[1 1 1] Mario hasn't entered transition level and entered level 1 dungeon
        (Variables|/Game/MarioGameInstance.MarioGameInstance_C|SetEnteredLevel1Pipe (Variables|Default|GetAs%20Mario%20Game%20Instance) false)
        (Variables|/Game/MarioGameInstance.MarioGameInstance_C|SetExitLevel1Pipe (Variables|Default|GetAs%20Mario%20Game%20Instance) true)
        (bind _outactor_4 (Sequencer|Player|CreateLevelSequencePlayer "/Game/Sequences/ExitDungeonSequencee.ExitDungeonSequencee"))
        (Sequencer|Player|Play (Variables|/Script/LevelSequence.LevelSequenceActor|GetSequencePlayer _outactor_4) :!class /Script/MovieScene.MovieSceneSequencePlayer)
        (Rendering|SetActorHiddenInGame (Variables|Default|GetMario) true)
        (Utilities|FlowControl|Delay 2.05)
        (Game|OpenLevel(byName) "Main" false)))))

(fn ConstructionScript)