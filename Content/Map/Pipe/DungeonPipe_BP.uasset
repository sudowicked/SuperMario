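; DungeonPipe_BP is a pipe actor that Mario can trigger by pressing S while standing within its capsule.
; The capsule's overlap events enable and disable the pipe's own input, so the key only responds when Mario is there.
; Pressing S briefly halts Mario, launches him upward with a backflip, then disables the pipe top's collision and player input, apparently so he drops into the pipe.
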(event OnComponentBeginOverlap(Capsule)
  (params (OverlappedComponent :type Primitive%20Component%20Object%20Reference) (OtherActor :type Actor%20Object%20Reference) (OtherComp :type Primitive%20Component%20Object%20Reference) (OtherBodyIndex :type Integer) (bFromSweep :type Boolean) (SweepResult :type Hit%20Result%20Structure%20%28by%20ref%29))
  (Utilities|Casting|CastToMario_BP OtherActor)
  (Input|EnableInput (Game|GetPlayerController 0)))

(event OnComponentEndOverlap(Capsule)
  (params (OverlappedComponent :type Primitive%20Component%20Object%20Reference) (OtherActor :type Actor%20Object%20Reference) (OtherComp :type Primitive%20Component%20Object%20Reference) (OtherBodyIndex :type Integer))
  (Utilities|Casting|CastToMario_BP OtherActor)
  (Input|DisableInput (Game|GetPlayerController 0)))

(event EventBeginPlay)

(event Input|KeyboardEvents|S
  (params (Key :type Key%20Structure :default "None"))
  (:Pressed
    (bind _returnvalue (Actor|GetActorOfClass "/Game/Characters/Mario/Mario_BP.Mario_BP_C"))
    (Pawn|Components|CharacterMovement|DisableMovement (Variables|/Script/Engine.Character|GetCharacterMovement _returnvalue))
    (Utilities|FlowControl|Delay 0.1)
    (Pawn|Components|CharacterMovement|SetMovementMode (Variables|/Script/Engine.Character|GetCharacterMovement _returnvalue) "MOVE_Walking" 0)
    (Character|LaunchCharacter _returnvalue "0, 0,1500.000000" false false)
    (Default|BackflipAnimation _returnvalue)
    (Collision|SetCollisionEnabled (Variables|Default|GetTop) "NoCollision")
    (Input|DisableInput (Game|GetPlayerCharacter 0) 0)))

(fn ConstructionScript)