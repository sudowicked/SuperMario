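; Pipe actor that sends Mario into the Level1_Dungeon level.
; Overlapping its capsule enables the pipe's input, so pressing S fires a one-shot entry and records EnteredFirstPipe in MarioGameInstance.
; A delay-timed chain launches Mario upward with an animation, disables top collision and player input, plays a level sequence and sound, resets his scale and hides him, then opens the dungeon.
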(event OnComponentBeginOverlap(Capsule)
  (params (OverlappedComponent :type Primitive%20Component%20Object%20Reference) (OtherActor :type Actor%20Object%20Reference) (OtherComp :type Primitive%20Component%20Object%20Reference) (OtherBodyIndex :type Integer) (bFromSweep :type Boolean) (SweepResult :type Hit%20Result%20Structure%20%28by%20ref%29))
  (Utilities|Casting|CastToMario_BP OtherActor)
  (Input|EnableInput (Game|GetPlayerController 0)))

(event OnComponentEndOverlap(Capsule)
  (params (OverlappedComponent :type Primitive%20Component%20Object%20Reference) (OtherActor :type Actor%20Object%20Reference) (OtherComp :type Primitive%20Component%20Object%20Reference) (OtherBodyIndex :type Integer))
  (Utilities|Casting|CastToMario_BP OtherActor)
  (Input|DisableInput (Game|GetPlayerController 0)))

(event EventBeginPlay)

(event Input|KeyboardEvents|S
  (params (Key :type Key%20Structure :default "None"))
  (:Pressed
    (Utilities|FlowControl|DoOnce false
      (:Completed
        (bind _asmario_game_instance (Utilities|Casting|CastToMarioGameInstance (Game|GetGameInstance)))
        (Variables|/Game/MarioGameInstance.MarioGameInstance_C|SetEnteredFirstPipe _asmario_game_instance true)
        (bind _returnvalue (Actor|GetActorOfClass "/Game/Characters/Mario/Mario_BP.Mario_BP_C"))
        (Pawn|Components|CharacterMovement|DisableMovement (Variables|/Script/Engine.Character|GetCharacterMovement _returnvalue))
        (Utilities|FlowControl|Delay 0.1)
        (Pawn|Components|CharacterMovement|SetMovementMode (Variables|/Script/Engine.Character|GetCharacterMovement _returnvalue) "MOVE_Walking" 0)
        (Character|LaunchCharacter _returnvalue "0, 0,1500.000000" false false)
        (Default|EnterPipeAnimation _returnvalue)
        (Collision|SetCollisionEnabled (Variables|Default|GetTopCollision) "NoCollision")
        (Input|DisableInput (Game|GetPlayerCharacter 0) 0)
        (Utilities|FlowControl|Delay 0.3)
        (bind _outactor (Sequencer|Player|CreateLevelSequencePlayer "/Game/Sequences/EnterDungeonSequenceMain.EnterDungeonSequenceMain"))
        (Sequencer|Player|Play (Variables|/Script/LevelSequence.LevelSequenceActor|GetSequencePlayer _outactor) :!class /Script/MovieScene.MovieSceneSequencePlayer)
        (Utilities|FlowControl|Delay 0.55)
        (Audio|PlaySound2D "/Game/Sound_Effects/PipeEnterExit.PipeEnterExit" 1.0 1.0 0.0 0 0)
        (Transformation|SetActorScale3D _returnvalue "1.000000,1.000000,1.000000")
        (Transformation|SetWorldScale3D (Variables|/Game/Characters/Mario/Mario_BP.Mario_BP_C|GetCameraBoom _returnvalue) "1.000000,1.000000,1.000000")
        (Rendering|SetActorHiddenInGame _returnvalue true)
        (Utilities|FlowControl|Delay 1.5)
        (Game|OpenLevel(byName) "Level1_Dungeon")))))

(fn ConstructionScript)