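; Brick block Blueprint that awards a coin and points through MarioGameInstance when Mario overlaps its collision.
; If MarioState is at least 1, it animates the coin, spawns a DestructibleBrickBlock_BP, adds points and destroys itself; otherwise it bumps and pops the coin.
; MoveComponentTo macros drive the motion; DoOnce limits only the coin sound, not the rewards.
; BeginPlay applies a blue material after the first pipe or Level 2 is entered.
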(event OnComponentBeginOverlap(Collision)
  (params (OverlappedComponent :type Primitive%20Component%20Object%20Reference) (OtherActor :type Actor%20Object%20Reference) (OtherComp :type Primitive%20Component%20Object%20Reference) (OtherBodyIndex :type Integer) (bFromSweep :type Boolean) (SweepResult :type Hit%20Result%20Structure%20%28by%20ref%29))
  (Utilities|Casting|CastToMario_BP OtherActor)
  (bind _asmario_game_instance (Utilities|Casting|CastToMarioGameInstance (Game|GetGameInstance)))
  (Default|AddCoin _asmario_game_instance)
  (Default|Add200Points _asmario_game_instance)
  (Utilities|FlowControl|Sequence
    (:then_0
      (Utilities|FlowControl|DoOnce false
        (:Completed
          (Audio|PlaySound2D "/Game/Sound_Effects/CoinSound.CoinSound" 1.0 1.0 0.0 0 0))))
    (:then_1
      (if (>= (Variables|/Game/MarioGameInstance.MarioGameInstance_C|GetMarioState _asmario_game_instance) 1)
        (Utilities|CoinMove/DestructibleBrickSpawn
          (:then
            (Utilities|FlowControl|Delay 0.01)
            (Components|DestroyComponent (Variables|Default|GetMario_Coin_BP))
            (Actor|DestroyActor)))
        (else
          (Audio|PlaySound2D "/Game/Sound_Effects/BumpSound.BumpSound" 1.0 1.0 0.0 0 0)
          (Utilities|Box/CoinMove
            (:then
              (Utilities|FlowControl|Delay 0.2)
              (Components|DestroyComponent (Variables|Default|GetMario_Coin_BP)))))))))

(event EventBeginPlay
  (bind _asmario_game_instance (Utilities|Casting|CastToMarioGameInstance (Game|GetGameInstance)))
  (if (or (Variables|/Game/MarioGameInstance.MarioGameInstance_C|GetEnteredFirstPipe _asmario_game_instance) (Variables|/Game/MarioGameInstance.MarioGameInstance_C|GetEnteredLevel2 _asmario_game_instance))
    (bind _returnvalue (Rendering|Material|CreateDynamicMaterialInstance (Variables|Default|GetBrick) 0 "/Game/Map/Boxes/BrickBox/BrickBlue_Material.BrickBlue_Material" "None" :!class /Script/Engine.PrimitiveComponent))
    (Rendering|Material|SetMaterial (Variables|Default|GetBrick) 0 _returnvalue)))

(fn ConstructionScript)