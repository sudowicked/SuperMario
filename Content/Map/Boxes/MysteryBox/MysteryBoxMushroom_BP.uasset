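; Mystery box Blueprint that releases a mushroom power-up when Mario overlaps its collision.
; On overlap it reveals the empty box, destroys the mystery mesh and collision so it fires only once, and plays the power-up appearing sound.
; The Box/MushroomMove graph spawns Mushroom_BP at an arrow's transform, then bumps the empty box up and back down with two quick MoveComponentTo moves.
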(event OnComponentBeginOverlap(Collision)
  (params (OverlappedComponent :type Primitive%20Component%20Object%20Reference) (OtherActor :type Actor%20Object%20Reference) (OtherComp :type Primitive%20Component%20Object%20Reference) (OtherBodyIndex :type Integer) (bFromSweep :type Boolean) (SweepResult :type Hit%20Result%20Structure%20%28by%20ref%29))
  (Utilities|Casting|CastToMario_BP OtherActor)
  (Development|SetHiddeninGame (Variables|Default|GetEmptyBox) false false)
  (Components|DestroyComponent (Variables|Default|GetMystery))
  (Audio|PlaySound2D "/Game/Sound_Effects/PowerUpAppearingSound.PowerUpAppearingSound" 1.0 1.0 0.0 0 0)
  (Utilities|Box/MushroomMove)
  (Components|DestroyComponent (Variables|Default|GetCollision)))

(event EventBeginPlay)

(event Collision|EventActorBeginOverlap
  (params (OtherActor :type Actor%20Object%20Reference)))

(event EventTick
  (params (DeltaSeconds :type Float%20%28single-precision%29)))

(fn ConstructionScript)