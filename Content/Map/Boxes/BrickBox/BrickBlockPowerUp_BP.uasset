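; Brick block that releases a power-up when Mario hits its trigger, knocking him downward and swapping the brick for an empty box.
; MarioState from the game instance selects a FireFlower or Mushroom spawn at the Arrow, with a short box bounce before the empty box's bump collision is enabled.
; Later hits on the empty box only push Mario down with a bump sound.
; On BeginPlay, the brick turns blue in the level 1 pipe area or level 2.
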(event OnComponentBeginOverlap(Collision)
  (params (OverlappedComponent :type Primitive%20Component%20Object%20Reference) (OtherActor :type Actor%20Object%20Reference) (OtherComp :type Primitive%20Component%20Object%20Reference) (OtherBodyIndex :type Integer) (bFromSweep :type Boolean) (SweepResult :type Hit%20Result%20Structure%20%28by%20ref%29))
  (bind _asmario_bp (Utilities|Casting|CastToMario_BP OtherActor))
  (Character|LaunchCharacter _asmario_bp "0, 0,-500.000000" false true)
  (Development|SetHiddeninGame (Variables|Default|GetEmptyBox) false false)
  (Components|DestroyComponent (Variables|Default|GetBrickblock))
  (Components|DestroyComponent (Variables|Default|GetCollision))
  (Audio|PlaySound2D "/Game/Sound_Effects/PowerUpAppearingSound.PowerUpAppearingSound" 1.0 1.0 0.0 0 0)
  (bind _asmario_game_instance (Utilities|Casting|CastToMarioGameInstance (Game|GetGameInstance)))
  (if (or (== (Variables|/Game/MarioGameInstance.MarioGameInstance_C|GetMarioState _asmario_game_instance) 1) (== (Variables|/Game/MarioGameInstance.MarioGameInstance_C|GetMarioState _asmario_game_instance) 2))
    (Utilities|Box/FlowerMove
      (:Completed
        (Collision|SetCollisionEnabled (Variables|Default|GetEmptyBoxCollsion) "QueryAndPhysics")))
    (else
      (Utilities|Box/MushroomMove
        (:Completed
          (Collision|SetCollisionEnabled (Variables|Default|GetEmptyBoxCollsion) "QueryAndPhysics"))))))

(event OnComponentBeginOverlap(EmptyBoxCollsion)
  (params (OverlappedComponent :type Primitive%20Component%20Object%20Reference) (OtherActor :type Actor%20Object%20Reference) (OtherComp :type Primitive%20Component%20Object%20Reference) (OtherBodyIndex :type Integer) (bFromSweep :type Boolean) (SweepResult :type Hit%20Result%20Structure%20%28by%20ref%29))
  (bind _asmario_bp (Utilities|Casting|CastToMario_BP OtherActor))
  (Character|LaunchCharacter _asmario_bp "0, 0,-500.000000" false true)
  (Audio|PlaySound2D "/Game/Sound_Effects/BumpSound.BumpSound" 1.0 1.0 0.0 0 0))

(event EventBeginPlay
  ;[1 1 1] Checking if mario is in dungeon or level 2 in order to change texture
  (bind _asmario_game_instance (Utilities|Casting|CastToMarioGameInstance (Game|GetGameInstance)))
  (if (or (Variables|/Game/MarioGameInstance.MarioGameInstance_C|GetEnteredLevel1Pipe _asmario_game_instance) (Variables|/Game/MarioGameInstance.MarioGameInstance_C|GetEnteredLevel2 _asmario_game_instance))
    (bind _returnvalue (Rendering|Material|CreateDynamicMaterialInstance (Variables|Default|GetBrickblock) 0 "/Game/Map/Boxes/BrickBox/BrickBlue_Material.BrickBlue_Material" "None" :!class /Script/Engine.PrimitiveComponent))
    (Rendering|Material|SetMaterial (Variables|Default|GetBrickblock) 0 _returnvalue)
    (Collision|SetCollisionEnabled (Variables|Default|GetEmptyBoxCollsion) "NoCollision")))

(fn ConstructionScript)