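; Mario brick block with a coin that bumps or breaks when Mario hits it, using blue material in the level 1 pipe area and level 2.
; Box overlap spawns a destructible brick and awards points for big Mario, or bumps brick and coin for small Mario.
; Coin overlap awards coin and points, then animates and removes the coin.
; MarioDetection overlap disables that coin trigger, preventing a repeat coin sound.
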(event OnComponentBeginOverlap(BoxMoveCollision)
  (params (OverlappedComponent :type Primitive%20Component%20Object%20Reference) (OtherActor :type Actor%20Object%20Reference) (OtherComp :type Primitive%20Component%20Object%20Reference) (OtherBodyIndex :type Integer) (bFromSweep :type Boolean) (SweepResult :type Hit%20Result%20Structure%20%28by%20ref%29))
  ;[1 1 1] On collision with mario checking if mario is big (spawns breakable break) or small (calls move box function)
  (Utilities|Casting|CastToMario_BP OtherActor)
  (bind _asmario_game_instance (Utilities|Casting|CastToMarioGameInstance (Game|GetGameInstance)))
  (if (>= (Variables|/Game/MarioGameInstance.MarioGameInstance_C|GetMarioState _asmario_game_instance) 1)
    (Utilities|DestructibleBrickSpawn
      (:then
        (Utilities|FlowControl|Delay 0.01)
        (Actor|DestroyActor)))
    (else
      (Audio|PlaySound2D "/Game/Sound_Effects/BumpSound.BumpSound" 1.0 1.0 0.0 0 0)
      (Utilities|BoxMove))))

(event OnComponentBeginOverlap(CoinMoveCollision)
  (params (OverlappedComponent :type Primitive%20Component%20Object%20Reference) (OtherActor :type Actor%20Object%20Reference) (OtherComp :type Primitive%20Component%20Object%20Reference) (OtherBodyIndex :type Integer) (bFromSweep :type Boolean) (SweepResult :type Hit%20Result%20Structure%20%28by%20ref%29))
  ;[1 1 1] Moving the coin upwards and downwards when mario collides with CoinMoveCollision
  (Utilities|Casting|CastToMario_BP OtherActor)
  (bind _asmario_game_instance (Utilities|Casting|CastToMarioGameInstance (Game|GetGameInstance)))
  (Default|AddCoin _asmario_game_instance)
  (Default|Add200Points _asmario_game_instance)
  (Audio|PlaySound2D "/Game/Sound_Effects/CoinSound.CoinSound" 1.0 1.0 0.0 0 0)
  (Components|DestroyComponent (Variables|Default|GetCoinMoveCollision))
  (Utilities|CoinMove
    (:then
      (Components|DestroyComponent (Variables|Default|GetMario_Coin_BP)))))

(event OnComponentBeginOverlap(MarioDetection)
  (params (OverlappedComponent :type Primitive%20Component%20Object%20Reference) (OtherActor :type Actor%20Object%20Reference) (OtherComp :type Primitive%20Component%20Object%20Reference) (OtherBodyIndex :type Integer) (bFromSweep :type Boolean) (SweepResult :type Hit%20Result%20Structure%20%28by%20ref%29))
  ;[1 1 1] Detecting if mario has taken coin so that coin sound doesnt play
  (Utilities|Casting|CastToMario_BP OtherActor)
  (Components|DestroyComponent (Variables|Default|GetCoinMoveCollision)))

(event EventBeginPlay
  ;[1 1 1] Checking if mario is in dungeon or level 2 in order to change texture
  (bind _asmario_game_instance (Utilities|Casting|CastToMarioGameInstance (Game|GetGameInstance)))
  (if (or (Variables|/Game/MarioGameInstance.MarioGameInstance_C|GetEnteredLevel1Pipe _asmario_game_instance) (Variables|/Game/MarioGameInstance.MarioGameInstance_C|GetEnteredLevel2 _asmario_game_instance))
    (bind _returnvalue (Rendering|Material|CreateDynamicMaterialInstance (Variables|Default|GetBrick) 0 "/Game/Map/Boxes/BrickBox/BrickBlue_Material.BrickBlue_Material" "None" :!class /Script/Engine.PrimitiveComponent))
    (Rendering|Material|SetMaterial (Variables|Default|GetBrick) 0 _returnvalue)))

(fn ConstructionScript)