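; Blue destructible brick block that acts as the shattering stage of a breakable box.
; BeginPlay plays the break sound, then after a short delay switches the destructible mesh to physics-only collision; a trailing delay leads to nothing.
; A MoveBox macro defines a quick up-and-down bump with two timed component moves, but the event graph never uses it.
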(event EventBeginPlay
  (Audio|PlaySound2D "/Game/Sound_Effects/BreakBlockSound.BreakBlockSound" 1.0 1.0 0.0 0 0)
  (Utilities|FlowControl|Delay 0.1)
  (Collision|SetCollisionEnabled (Variables|Default|GetBrickBlock_StaticMesh_DM) "PhysicsOnly")
  (Utilities|FlowControl|Delay 0.6))

(event Collision|EventActorBeginOverlap
  (params (OtherActor :type Actor%20Object%20Reference)))

(event EventTick
  (params (DeltaSeconds :type Float%20%28single-precision%29)))

(fn ConstructionScript)