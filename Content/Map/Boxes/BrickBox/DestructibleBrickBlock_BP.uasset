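; Destructible brick block for a Mario-style game that plays its break sound as soon as it begins play.
; BeginPlay applies a blue dynamic material if the game instance flags the first pipe or level 2 as entered.
; After a short delay it switches the mesh to physics-only collision; a trailing delay leads to nothing.
; A MoveBox graph, not called here, defines a quick up-and-down bump through chained MoveComponentTo nodes.
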(event EventBeginPlay
  (Utilities|FlowControl|Sequence
    (:then_0
      (bind _asmario_game_instance (Utilities|Casting|CastToMarioGameInstance (Game|GetGameInstance)))
      (if (or (Variables|/Game/MarioGameInstance.MarioGameInstance_C|GetEnteredFirstPipe _asmario_game_instance) (Variables|/Game/MarioGameInstance.MarioGameInstance_C|GetEnteredLevel2 _asmario_game_instance))
        (bind _returnvalue (Rendering|Material|CreateDynamicMaterialInstance (Variables|Default|GetBrickBlock_StaticMesh_DM) 0 "/Game/Map/Boxes/BrickBox/BrickBlue_Material.BrickBlue_Material" "None" :!class /Script/Engine.PrimitiveComponent))
        (Rendering|Material|SetMaterial (Variables|Default|GetBrickBlock_StaticMesh_DM) 0 _returnvalue)))
    (:then_1
      (Audio|PlaySound2D "/Game/Sound_Effects/BreakBlockSound.BreakBlockSound" 1.0 1.0 0.0 0 0)
      (Utilities|FlowControl|Delay 0.1)
      (Collision|SetCollisionEnabled (Variables|Default|GetBrickBlock_StaticMesh_DM) "PhysicsOnly")
      (Utilities|FlowControl|Delay 0.6))))

(fn ConstructionScript)