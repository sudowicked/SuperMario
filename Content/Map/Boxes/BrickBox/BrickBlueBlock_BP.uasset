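; Blue brick block for a Mario-style game that reacts when Mario hits it.
; On overlap with its Collision component, it casts the other actor to Mario_BP and checks the BigMario flag.
; Big Mario swaps it for a DestructibleBrickBlock_BP spawned at the same transform.
; Otherwise it plays a sound and the MoveBox graph bumps the Brick component briefly up and back down using MoveComponentTo.
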(event OnComponentBeginOverlap(Collision)
  (params (OverlappedComponent :type Primitive%20Component%20Object%20Reference) (OtherActor :type Actor%20Object%20Reference) (OtherComp :type Primitive%20Component%20Object%20Reference) (OtherBodyIndex :type Integer) (bFromSweep :type Boolean) (SweepResult :type Hit%20Result%20Structure%20%28by%20ref%29))
  (bind _asmario_bp (Utilities|Casting|CastToMario_BP OtherActor))
  (if (Variables|/Game/Characters/Mario/Mario_BP.Mario_BP_C|GetBigMario _asmario_bp)
    (Actor|DestroyActor)
    (Game|SpawnActorfromClass "/Game/Map/Boxes/BrickBox/DestructibleBrickBlock_BP.DestructibleBrickBlock_BP_C" (Transformation|GetActorTransform) "Undefined" 0 0)
    (else
      (Audio|PlaySound2D 0 1.0 1.0 0.0 0 0)
      (Utilities|MoveBox))))

(event EventBeginPlay)

(event Collision|EventActorBeginOverlap
  (params (OtherActor :type Actor%20Object%20Reference)))

(event EventTick
  (params (DeltaSeconds :type Float%20%28single-precision%29)))

(fn ConstructionScript)