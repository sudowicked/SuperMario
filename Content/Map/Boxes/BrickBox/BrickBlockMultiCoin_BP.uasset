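; Multi-coin brick block that Mario hits repeatedly for coins and points until it becomes a solid empty box on the eighth hit.
; Overlaps push Mario down, count hits and show points text; earlier hits award coins and score.
; The Box/CoinMove graph bumps the block, reverses any mushroom on top and animates one coin per hit through a non-looping MultiGate.
; BeginPlay swaps to blue brick in the pipe area or level 2.
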(event OnComponentBeginOverlap(EmptyBoxCollsion)
  (params (OverlappedComponent :type Primitive%20Component%20Object%20Reference) (OtherActor :type Actor%20Object%20Reference) (OtherComp :type Primitive%20Component%20Object%20Reference) (OtherBodyIndex :type Integer) (bFromSweep :type Boolean) (SweepResult :type Hit%20Result%20Structure%20%28by%20ref%29))
  ;[1 1 1] Play sound on EmptyBoxCollision with mario
  (bind _asmario_bp (Utilities|Casting|CastToMario_BP OtherActor))
  (Character|LaunchCharacter _asmario_bp "0, 0,-500.000000" false true)
  (Audio|PlaySound2D "/Game/Sound_Effects/BumpSound.BumpSound" 1.0 1.0 0.0 0 0))

(event OnComponentBeginOverlap(Collision)
  (params (OverlappedComponent :type Primitive%20Component%20Object%20Reference) (OtherActor :type Actor%20Object%20Reference) (OtherComp :type Primitive%20Component%20Object%20Reference) (OtherBodyIndex :type Integer) (bFromSweep :type Boolean) (SweepResult :type Hit%20Result%20Structure%20%28by%20ref%29))
  ;[1 1 1] Moving box and coin upwards and downwards on mario collision/spawning empty box texture
  (bind _asmario_bp (Utilities|Casting|CastToMario_BP OtherActor))
  (Variables|Default|SetCoinCounter (+ (Variables|Default|GetCoinCounter) 1))
  (Character|LaunchCharacter _asmario_bp "0, 0,-500.000000" false true)
  (Utilities|FlowControl|Sequence
    (:then_0
      (if (== (Variables|Default|GetCoinCounter) 8)
        (Components|DestroyComponent (Variables|Default|GetCollision))
        (Development|SetHiddeninGame (Variables|Default|GetBrick) true false)
        (Development|SetHiddeninGame (Variables|Default|GetEmptyBox) false false)
        (Collision|SetCollisionEnabled (Variables|Default|GetEmptyBoxCollsion) "QueryAndPhysics")
        (Utilities|Box/CoinMove)
        (else
          (bind _asmario_game_instance (Utilities|Casting|CastToMarioGameInstance (Game|GetGameInstance)))
          (Default|AddCoin _asmario_game_instance)
          (Default|Add200Points _asmario_game_instance)
          (Audio|PlaySound2D "/Game/Sound_Effects/CoinSound.CoinSound" 1.0 1.0 0.0 0 0)
          (Utilities|Box/CoinMove))))
    (:then_1
      (CallFunction|PointsText))))

(event EventBeginPlay
  ;[1 1 1] Checking if mario is in dungeon or level 2 in order to change texture
  (bind _asmario_game_instance (Utilities|Casting|CastToMarioGameInstance (Game|GetGameInstance)))
  (if (or (Variables|/Game/MarioGameInstance.MarioGameInstance_C|GetEnteredLevel1Pipe _asmario_game_instance) (Variables|/Game/MarioGameInstance.MarioGameInstance_C|GetEnteredLevel2 _asmario_game_instance))
    (bind _returnvalue (Rendering|Material|CreateDynamicMaterialInstance (Variables|Default|GetBrick) 0 "/Game/Map/Boxes/BrickBox/BrickBlue_Material.BrickBlue_Material" "None" :!class /Script/Engine.PrimitiveComponent))
    (Rendering|Material|SetMaterial (Variables|Default|GetBrick) 0 _returnvalue)))

(fn ConstructionScript)

(fn PointsText
  (bind _returnvalue (Transformation|GetActorTransform))
  (bind _returnvalue_2 (Game|SpawnActorfromClass "/Game/Characters/PointsText_BP.PointsText_BP_C" (Math|Transform|MakeTransform (Math|Vector|MakeVector (.x (.location _returnvalue)) (+ (.y (.location _returnvalue)) 1e+02) (+ (.z (.location _returnvalue)) 2e+02)) "0,90.000000, 0" "1,1,1") "Undefined" 0 0))
  (bind _returnvalue_3 (UserInterface|CreateWidget "/Game/HUD/Points_Text/200_Points_Widget.200_Points_Widget_C"))
  (UserInterface|SetWidget (Variables|/Game/Characters/PointsText_BP.PointsText_BP_C|GetPoints _returnvalue_2) _returnvalue_3))