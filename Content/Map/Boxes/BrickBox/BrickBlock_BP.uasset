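; Breakable brick block for a Mario game that turns blue once the game instance flags the first pipe or level 2 as entered.
; Mario's overlap breaks it when MarioState is at least 1, spawning DestructibleBrickBlock_BP and awarding points; otherwise it bumps with a sound.
; GoombaDetection caches an overlapping Goomba for delayed removal on break, but the brick destroys itself before that delay ends.
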(event OnComponentBeginOverlap(GoombaDetection)
  (params (OverlappedComponent :type Primitive%20Component%20Object%20Reference) (OtherActor :type Actor%20Object%20Reference) (OtherComp :type Primitive%20Component%20Object%20Reference) (OtherBodyIndex :type Integer) (bFromSweep :type Boolean) (SweepResult :type Hit%20Result%20Structure%20%28by%20ref%29))
  (bind _asgoomba_bp (Utilities|Casting|CastToGoomba_BP OtherActor))
  (Variables|Default|SetAs%20Goomba%20BP _asgoomba_bp)
  (Variables|Default|SetOnBrick true))

(event OnComponentBeginOverlap(Collision)
  (params (OverlappedComponent :type Primitive%20Component%20Object%20Reference) (OtherActor :type Actor%20Object%20Reference) (OtherComp :type Primitive%20Component%20Object%20Reference) (OtherBodyIndex :type Integer) (bFromSweep :type Boolean) (SweepResult :type Hit%20Result%20Structure%20%28by%20ref%29))
  (Utilities|Casting|CastToMario_BP OtherActor)
  (bind _asmario_game_instance (Utilities|Casting|CastToMarioGameInstance (Game|GetGameInstance)))
  (if (>= (Variables|/Game/MarioGameInstance.MarioGameInstance_C|GetMarioState _asmario_game_instance) 1)
    (Utilities|FlowControl|Sequence
      (:then_0
        (Game|SpawnActorfromClass "/Game/Map/Boxes/BrickBox/DestructibleBrickBlock_BP.DestructibleBrickBlock_BP_C" (Transformation|GetActorTransform) "Undefined" 0 0)
        (Default|Add50Points _asmario_game_instance)
        (Utilities|FlowControl|Delay 0.1)
        (Actor|DestroyActor))
      (:then_1
        (Utilities|FlowControl|Delay 0.6)
        (Actor|DestroyActor (Variables|Default|GetAs%20Goomba%20BP))))
    (else
      (Audio|PlaySound2D "/Game/Sound_Effects/BumpSound.BumpSound" 1.0 1.0 0.0 0 0)
      (Utilities|MoveBox))))

(event OnComponentEndOverlap(GoombaDetection)
  (params (OverlappedComponent :type Primitive%20Component%20Object%20Reference) (OtherActor :type Actor%20Object%20Reference) (OtherComp :type Primitive%20Component%20Object%20Reference) (OtherBodyIndex :type Integer))
  (Utilities|Casting|CastToGoomba_BP OtherActor)
  (Variables|Default|SetOnBrick false))

(event EventBeginPlay
  (bind _asmario_game_instance (Utilities|Casting|CastToMarioGameInstance (Game|GetGameInstance)))
  (if (or (Variables|/Game/MarioGameInstance.MarioGameInstance_C|GetEnteredFirstPipe _asmario_game_instance) (Variables|/Game/MarioGameInstance.MarioGameInstance_C|GetEnteredLevel2 _asmario_game_instance))
    (bind _returnvalue (Rendering|Material|CreateDynamicMaterialInstance (Variables|Default|GetBrick) 0 "/Game/Map/Boxes/BrickBox/BrickBlue_Material.BrickBlue_Material" "None" :!class /Script/Engine.PrimitiveComponent))
    (Rendering|Material|SetMaterial (Variables|Default|GetBrick) 0 _returnvalue)))

(fn ConstructionScript)