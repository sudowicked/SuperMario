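; Menu_BP is a menu actor with a widget component, linked to other menus that the player's view moves between.
; On BeginPlay it disables its collision and binds to the transition event on its Menu_Widget.
; A transition disables its own collision, cubic-blends the view target to the indexed linked menu, then enables that menu's collision after a matching delay.
; The validity guard checks only index zero, not the requested index.
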(event Custom|TransitionTo
  (params (NewMenu :type Menu%20BP%20Object%20Reference))
  (Collision|SetActorEnableCollision false)
  (Game|Player|SetViewTargetwithBlend (Game|GetPlayerController 0) NewMenu 3.0 "VTBlend_Cubic" 3.0 false)
  (Utilities|FlowControl|Delay 3.0)
  (Collision|SetActorEnableCollision NewMenu true))

(event Custom|OnTransitionBetweenMenus
  (params (MenuIndex :type Integer))
  (if (Utilities|Array|IsValidIndex (Variables|Default|GetLinkedMenus))
    (CallFunction|Transitionto (Utilities|Array|Get(acopy) (Variables|Default|GetLinkedMenus) MenuIndex))))

(event EventBeginPlay
  (bind _asmenu_widget (Utilities|Casting|CastToMenu_Widget (UserInterface|GetUserWidgetObject (Variables|Default|GetWidget))))
  (EventDispatchers|BindEventtoTransitiontoLinkedMenu _asmenu_widget (delegate Custom|OnTransitionBetweenMenus))
  (Collision|SetActorEnableCollision false))

(fn ConstructionScript)