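; Koopa enemy character that walks back and forth and turns into a shell when Mario touches its collision component.
; It spawns a default controller on BeginPlay and adds movement input every tick along its MovementDirection.
; Hits on actors tagged HitActor trigger a FlipFlop that alternates its facing and X direction.
; A Mario_BP overlap on Collision spawns Koopa_Shell_BP at its transform and destroys the Koopa.
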(event OnComponentBeginOverlap(Collision)
  (params (OverlappedComponent :type Primitive%20Component%20Object%20Reference) (OtherActor :type Actor%20Object%20Reference) (OtherComp :type Primitive%20Component%20Object%20Reference) (OtherBodyIndex :type Integer) (bFromSweep :type Boolean) (SweepResult :type Hit%20Result%20Structure%20%28by%20ref%29))
  (Utilities|Casting|CastToMario_BP OtherActor)
  (Game|SpawnActorfromClass "/Game/Characters/Koopa/Koopa_Shell_BP.Koopa_Shell_BP_C" (Transformation|GetActorTransform) "Undefined" 0 0)
  (Actor|DestroyActor))

(event EventBeginPlay
  (Pawn|SpawnDefaultController))

(event Collision|EventActorBeginOverlap
  (params (OtherActor :type Actor%20Object%20Reference)))

(event EventTick
  (params (DeltaSeconds :type Float%20%28single-precision%29))
  (Pawn|Input|AddMovementInput (Variables|Default|GetMovementDirection) 0.4 false))

(event Collision|EventHit
  (params (MyComp :type Primitive%20Component%20Object%20Reference) (Other :type Actor%20Object%20Reference) (OtherComp :type Primitive%20Component%20Object%20Reference) (bSelfMoved :type Boolean) (HitLocation :type Vector :default "0, 0, 0") (HitNormal :type Vector :default "0, 0, 0") (NormalImpulse :type Vector :default "0, 0, 0") (Hit :type Hit%20Result%20Structure%20%28by%20ref%29))
  (if (Actor|ActorHasTag Other "HitActor")
    (Utilities|FlowControl|FlipFlop
      (:A
        (Transformation|SetActorRelativeRotation "0,-90.000000, 0")
        (Variables|Default|SetMovementDirection "1.000000,0.000000, 0"))
      (:B
        (Transformation|SetActorRelativeRotation "0,90.000000, 0")
        (Variables|Default|SetMovementDirection "-1.000000,0.000000, 0")))))

(fn ConstructionScript)