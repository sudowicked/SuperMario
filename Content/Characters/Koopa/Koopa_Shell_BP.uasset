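; Koopa shell character that Mario kicks into a spinning slide, earning points, and that then becomes a hazard.
; Front or back component hits set the direction Tick drives via movement input, and nested FlipFlops flip it on "HitActor"-tagged hits.
; Capsule overlap kills or powers down Mario by game-instance state, with temporary pass-through afterward.
; Fireballs, Star Mario or a just-hit Mario trigger its flip-and-drop death.
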(event OnComponentBeginOverlap(CapsuleComponent)
  (params (OverlappedComponent :type Primitive%20Component%20Object%20Reference) (OtherActor :type Actor%20Object%20Reference) (OtherComp :type Primitive%20Component%20Object%20Reference) (OtherBodyIndex :type Integer) (bFromSweep :type Boolean) (SweepResult :type Hit%20Result%20Structure%20%28by%20ref%29))
  ;[1 1 1] Death if hit by mario in star form/power down or kill mario if he is in default state
  (bind _asmario_bp (Utilities|Casting|CastToMario_BP OtherActor))
  (Variables|Default|SetAs%20Mario%20BP _asmario_bp)
  (bind _asmario_game_instance (Utilities|Casting|CastToMarioGameInstance (Game|GetGameInstance)))
  (bind _output_get (Variables|Default|SetMario%20Game%20Instance _asmario_game_instance))
  (if (or (Variables|/Game/MarioGameInstance.MarioGameInstance_C|GetStarMario _asmario_game_instance) (Variables|/Game/MarioGameInstance.MarioGameInstance_C|GetMarioWasJustHit _asmario_game_instance))
    (CallFunction|DeathbyFireball/StarMario)
    (Utilities|FlowControl|DoOnce false
      (:Completed
        (Audio|PlaySound2D "/Game/Sound_Effects/StompSound.StompSound" 1.0 1.0 0.0 0 0)))
    (elif (== (Variables|/Game/MarioGameInstance.MarioGameInstance_C|GetMarioState _output_get) 0)
      (Default|MarioDeath (Variables|Default|GetAs%20Mario%20BP))
      (elif (== (Variables|/Game/MarioGameInstance.MarioGameInstance_C|GetMarioState _output_get) 1)
        (Default|PowerDown (Variables|Default|GetAs%20Mario%20BP))
        (Collision|SetCollisionResponsetoChannel (Variables|/Script/Engine.Character|GetCapsuleComponent (Variables|Default|GetAs%20Mario%20BP)) "ECC_Pawn" "ECR_Overlap")
        (Variables|/Game/MarioGameInstance.MarioGameInstance_C|SetMarioWasJustHit (Variables|Default|GetMario%20Game%20Instance) true)
        (Utilities|FlowControl|Delay 3.0)
        (Variables|/Game/MarioGameInstance.MarioGameInstance_C|SetMarioWasJustHit (Variables|Default|GetMario%20Game%20Instance) false)
        (Collision|SetCollisionResponsetoChannel (Variables|Collision|GetCapsuleComponent) "ECC_Pawn" "ECR_Block")
        (else
          (Default|CookPowerDowntoMario (Variables|Default|GetAs%20Mario%20BP))
          (Collision|SetCollisionResponsetoChannel (Variables|Collision|GetCapsuleComponent) "ECC_Pawn" "ECR_Overlap")
          (Variables|/Game/MarioGameInstance.MarioGameInstance_C|SetMarioWasJustHit (Variables|Default|GetMario%20Game%20Instance) true)
          (Utilities|FlowControl|Delay 3.0)
          (Variables|/Game/MarioGameInstance.MarioGameInstance_C|SetMarioWasJustHit (Variables|Default|GetMario%20Game%20Instance) false)
          (Collision|SetCollisionResponsetoChannel (Variables|Collision|GetCapsuleComponent) "ECC_Pawn" "ECR_Block"))))))

(event OnComponentHit(Back_Collision)
  (params (HitComponent :type Primitive%20Component%20Object%20Reference) (OtherActor :type Actor%20Object%20Reference) (OtherComp :type Primitive%20Component%20Object%20Reference) (NormalImpulse :type Vector :default "0, 0, 0") (Hit :type Hit%20Result%20Structure%20%28by%20ref%29))
  ;[1 1 1] Shell begins to accelerate when mario kicks it either on the front or the back
  (bind _asmario_game_instance (Utilities|Casting|CastToMarioGameInstance (Game|GetGameInstance)))
  (if (not (Variables|/Game/MarioGameInstance.MarioGameInstance_C|GetStarMario _asmario_game_instance))
    (Utilities|FlowControl|Sequence
      (:then_0
        (bind _asmario_bp (Utilities|Casting|CastToMario_BP OtherActor))
        (Audio|PlaySound2D "/Game/Sound_Effects/StompSound.StompSound" 1.0 1.0 0.0 0 0)
        (CallFunction|Spin)
        (Variables|Default|SetBackHit true)
        (Components|DestroyComponent (Variables|Default|GetFront_Collsion))
        (Variables|/Script/Engine.CharacterMovementComponent|SetBrakingDecelerationFalling (Variables|/Script/Engine.Character|GetCharacterMovement _asmario_bp) 1e+08)
        (Utilities|FlowControl|Delay 0.2)
        (Variables|/Script/Engine.CharacterMovementComponent|SetBrakingDecelerationFalling (Variables|/Script/Engine.Character|GetCharacterMovement _asmario_bp) 0.0))
      (:then_1
        (bind _asmario_bp_2 (Utilities|Casting|CastToMario_BP OtherActor))
        (bind _asmario_game_instance_2 (Utilities|Casting|CastToMarioGameInstance (Game|GetGameInstance)))
        (Default|Add200Points _asmario_game_instance_2)
        (Default|MarioKickAnimation _asmario_bp_2)
        (Utilities|FlowControl|Delay 0.5)
        (Default|MarioDefaultAnimation _asmario_bp_2)))))

(event OnComponentHit(Front_Collsion)
  (params (HitComponent :type Primitive%20Component%20Object%20Reference) (OtherActor :type Actor%20Object%20Reference) (OtherComp :type Primitive%20Component%20Object%20Reference) (NormalImpulse :type Vector :default "0, 0, 0") (Hit :type Hit%20Result%20Structure%20%28by%20ref%29))
  ;[1 1 1] Shell begins to accelerate when mario kicks it either on the front or the back
  (bind _asmario_game_instance (Utilities|Casting|CastToMarioGameInstance (Game|GetGameInstance)))
  (if (not (Variables|/Game/MarioGameInstance.MarioGameInstance_C|GetStarMario _asmario_game_instance))
    (Utilities|FlowControl|Sequence
      (:then_0
        (bind _asmario_bp (Utilities|Casting|CastToMario_BP OtherActor))
        (Audio|PlaySound2D "/Game/Sound_Effects/StompSound.StompSound" 1.0 1.0 0.0 0 0)
        (CallFunction|Spin)
        (Variables|Default|SetFrontHit true)
        (Components|DestroyComponent (Variables|Default|GetFront_Collsion))
        (Variables|/Script/Engine.CharacterMovementComponent|SetBrakingDecelerationFalling (Variables|/Script/Engine.Character|GetCharacterMovement _asmario_bp) 1e+08)
        (Utilities|FlowControl|Delay 0.2)
        (Variables|/Script/Engine.CharacterMovementComponent|SetBrakingDecelerationFalling (Variables|/Script/Engine.Character|GetCharacterMovement _asmario_bp) 0.0))
      (:then_1
        (bind _asmario_bp_2 (Utilities|Casting|CastToMario_BP OtherActor))
        (bind _asmario_game_instance_2 (Utilities|Casting|CastToMarioGameInstance (Game|GetGameInstance)))
        (Default|Add200Points _asmario_game_instance_2)
        (Default|MarioKickAnimation _asmario_bp_2)
        (Utilities|FlowControl|Delay 0.5)
        (Default|MarioDefaultAnimation _asmario_bp_2)))))

(event Custom|DeathByFireball/Star%20Mario
  (bind _capsulecomponent (Variables|Collision|GetCapsuleComponent))
  (bind _capsulecomponent_2 (Variables|Collision|GetCapsuleComponent))
  (bind _relativelocation (Variables|/Script/Engine.SceneComponent|GetRelativeLocation _capsulecomponent))
  (bind _relativelocation_2 (Variables|/Script/Engine.SceneComponent|GetRelativeLocation _capsulecomponent_2))
  ;[1 1 1] Death by fire ball / star mario logic
  (Utilities|FlowControl|DoOnce false
    (:Completed
      (Components|MoveComponentTo _capsulecomponent_2 (Math|Vector|MakeVector (.x _relativelocation_2) (.y _relativelocation_2) (+ (.z _relativelocation_2) 4e+01)) "0.000000,90.000000,180.000000" false false 0.01 false)
      (Collision|SetCollisionEnabled _capsulecomponent "NoCollision")
      (Components|MoveComponentTo _capsulecomponent (Math|Vector|MakeVector (.x _relativelocation) (.y _relativelocation) (- (.z _relativelocation) 2e+02)) "0.000000,90.000000,180.000000" false false 0.4 false)
      (Actor|DestroyActor))))

(event EventBeginPlay
  ;[1 1 1] Making the actor movable
  (Pawn|SpawnDefaultController))

(event EventTick
  (params (DeltaSeconds :type Float%20%28single-precision%29))
  ;[1 1 1] Constantly adding movement after being kicked either on the front or the back
  (if (Variables|Default|GetFrontHit)
    (Pawn|Input|AddMovementInput (Variables|Default|GetMovementDirectionFront) 1e+01 false)
    (elif (Variables|Default|GetBackHit)
      (Pawn|Input|AddMovementInput (Variables|Default|GetMovementDirectionBack) 1e+01 false))))

(event Collision|EventActorBeginOverlap
  (params (OtherActor :type Actor%20Object%20Reference))
  ;[1 1 1] Death when hit by fireball
  (Utilities|Casting|CastToFireBall OtherActor)
  (CallFunction|DeathbyFireball/StarMario))

(event Collision|EventHit
  (params (MyComp :type Primitive%20Component%20Object%20Reference) (Other :type Actor%20Object%20Reference) (OtherComp :type Primitive%20Component%20Object%20Reference) (bSelfMoved :type Boolean) (HitLocation :type Vector :default "0, 0, 0") (HitNormal :type Vector :default "0, 0, 0") (NormalImpulse :type Vector :default "0, 0, 0") (Hit :type Hit%20Result%20Structure%20%28by%20ref%29))
  ;[1 1 1] Change direction when hitting certain objects
  (if (Actor|ActorHasTag Other "HitActor")
    (Utilities|FlowControl|FlipFlop
      (:A
        (Utilities|FlowControl|FlipFlop
          (:A
            (Variables|Default|SetMovementDirectionFront "1.000000, 0, 0"))
          (:B
            (Variables|Default|SetMovementDirectionBack "1.000000, 0, 0"))))
      (:B
        (Utilities|FlowControl|FlipFlop
          (:A
            (Variables|Default|SetMovementDirectionFront "-1.000000, 0, 0"))
          (:B
            (Variables|Default|SetMovementDirectionBack "-1.000000, 0, 0")))))))

(fn ConstructionScript)

(fn Spin
  (Components|Animation|PlayAnimation (Variables|Character|GetMesh) "/Game/Characters/Koopa/Animations/Koopa_Shell_Spin_Anim.Koopa_Shell_Spin_Anim" true))