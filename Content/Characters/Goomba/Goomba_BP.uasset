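; Goomba enemy character that walks along the X axis, flips direction on hitting tagged actors, and uses blue materials in level 2.
; Box hits from Mario stomp and squash it, while capsule hits kill, downgrade or briefly make Mario invulnerable based on game instance state.
; Fireballs, Koopa shells, Star Mario and a brick-hit trigger cause flip-over deaths with points.
; Each death path plays the death animation, moves the capsule and destroys the actor.
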(event OnComponentBeginOverlap(BrickHitCollision)
  (params (OverlappedComponent :type Primitive%20Component%20Object%20Reference) (OtherActor :type Actor%20Object%20Reference) (OtherComp :type Primitive%20Component%20Object%20Reference) (OtherBodyIndex :type Integer) (bFromSweep :type Boolean) (SweepResult :type Hit%20Result%20Structure%20%28by%20ref%29))
  (bind _returnvalue (Actor|GetComponentbyClass "/Script/Engine.CapsuleComponent"))
  (bind _charactermovement (Variables|Character|GetCharacterMovement))
  (bind _capsulecomponent (Variables|Collision|GetCapsuleComponent))
  (bind _returnvalue_2 (Transformation|GetWorldTransform _returnvalue))
  (bind _returnvalue_3 (Transformation|GetWorldTransform _capsulecomponent))
  ;[1 1 1] Death by brick hit
  (Utilities|Casting|CastToMario_BP OtherActor)
  (bind _asmario_game_instance (Utilities|Casting|CastToMarioGameInstance (Game|GetGameInstance)))
  (Default|Add100Points _asmario_game_instance)
  (if (not (Variables|/Game/MarioGameInstance.MarioGameInstance_C|GetMarioWasJustHit _asmario_game_instance))
    (if (AI|Components|NavMovement|IsMovingonGround (Variables|Character|GetCharacterMovement))
      (Components|MoveComponentTo (Variables|Collision|GetCapsuleComponent) (Math|Vector|MakeVector (.x (.location _returnvalue_2)) (.y (.location _returnvalue_2)) (+ (.z (.location _returnvalue_2)) 1e+02)) "180.000000,0.000000, 0" false false 0.01 false)
      (Components|Movement|StopMovementImmediately _charactermovement)
      (Pawn|Components|CharacterMovement|DisableMovement _charactermovement)
      (CallFunction|Death)
      (Components|MoveComponentTo _capsulecomponent (Math|Vector|MakeVector (.x (.location _returnvalue_3)) -2e+03 (- (.z (.location _returnvalue_3)) 6e+02)) (.rotation _returnvalue_3) false false 0.7 false)
      (Actor|DestroyActor))))

(event OnComponentHit(Box)
  (params (HitComponent :type Primitive%20Component%20Object%20Reference) (OtherActor :type Actor%20Object%20Reference) (OtherComp :type Primitive%20Component%20Object%20Reference) (NormalImpulse :type Vector :default "0, 0, 0") (Hit :type Hit%20Result%20Structure%20%28by%20ref%29))
  (bind _charactermovement (Variables|Character|GetCharacterMovement))
  (bind _capsulecomponent (Variables|Collision|GetCapsuleComponent))
  (bind _asmario_bp (Utilities|Casting|CastToMario_BP OtherActor))
  (bind _asmario_game_instance (Utilities|Casting|CastToMarioGameInstance (Game|GetGameInstance)))
  (Default|Add100Points _asmario_game_instance)
  (Utilities|FlowControl|DoOnce false
    (:Completed
      (Audio|PlaySound2D "/Game/Sound_Effects/StompSound.StompSound" 1.0 1.0 0.0 0 0)
      (Character|LaunchCharacter _asmario_bp "0.000000, 0,-200.000000" false false)
      (Collision|SetCollisionEnabled (Variables|Character|GetMesh) "NoCollision")
      (Components|Movement|StopMovementImmediately _charactermovement)
      (Pawn|Components|CharacterMovement|DisableMovement _charactermovement)
      (CallFunction|Death)
      (Transformation|SetWorldScale3D (Variables|Collision|GetCapsuleComponent) "1.000000,1.000000,0.500000")
      (Components|MoveComponentTo _capsulecomponent (+ (Variables|/Script/Engine.SceneComponent|GetRelativeLocation _capsulecomponent) "0, 0,-35.000000") "0, 0, 0" false false 0.2 false)
      (Utilities|FlowControl|Delay 0.2)
      (Actor|DestroyActor))))

(event OnComponentHit(CapsuleComponent)
  (params (HitComponent :type Primitive%20Component%20Object%20Reference) (OtherActor :type Actor%20Object%20Reference) (OtherComp :type Primitive%20Component%20Object%20Reference) (NormalImpulse :type Vector :default "0, 0, 0") (Hit :type Hit%20Result%20Structure%20%28by%20ref%29))
  (bind _asmario_bp (Utilities|Casting|CastToMario_BP OtherActor))
  (Variables|Default|SetAs%20Mario%20BP _asmario_bp)
  (bind _asmario_game_instance (Utilities|Casting|CastToMarioGameInstance (Game|GetGameInstance)))
  (bind _output_get (Variables|Default|SetMario%20Game%20Instance _asmario_game_instance))
  (if (not (Variables|/Game/MarioGameInstance.MarioGameInstance_C|GetMarioWasJustHit _asmario_game_instance))
    (if (Variables|/Game/MarioGameInstance.MarioGameInstance_C|GetStarMario _asmario_game_instance)
      (CallFunction|DeathbyFireball/StarMario/Koopa)
      (Default|Add100Points _asmario_game_instance)
      (Audio|PlaySound2D "/Game/Sound_Effects/StompSound.StompSound" 1.0 1.0 0.0 0 0)
      (elif (== (Variables|/Game/MarioGameInstance.MarioGameInstance_C|GetMarioState _output_get) 0)
        (Default|MarioDeath (Variables|Default|GetAs%20Mario%20BP))
        (elif (== (Variables|/Game/MarioGameInstance.MarioGameInstance_C|GetMarioState _output_get) 1)
          (Default|PowerDown (Variables|Default|GetAs%20Mario%20BP))
          (Collision|SetCollisionResponsetoChannel (Variables|/Script/Engine.Character|GetCapsuleComponent (Variables|Default|GetAs%20Mario%20BP)) "ECC_Pawn" "ECR_Overlap")
          (Variables|/Game/MarioGameInstance.MarioGameInstance_C|SetMarioWasJustHit (Variables|Default|GetMario%20Game%20Instance) true)
          (Default|InvulnerabilityAnimation (Variables|Default|GetAs%20Mario%20BP))
          (Utilities|FlowControl|Delay 3.0)
          (Variables|/Game/MarioGameInstance.MarioGameInstance_C|SetMarioWasJustHit (Variables|Default|GetMario%20Game%20Instance) false)
          (Collision|SetCollisionResponsetoChannel (Variables|Collision|GetCapsuleComponent) "ECC_Pawn" "ECR_Block")
          (Collision|SetCollisionResponsetoChannel (Variables|Default|GetBrickHitCollision) "ECC_Pawn" "ECR_Overlap")
          (else
            (Default|CooktoMario (Variables|Default|GetAs%20Mario%20BP))
            (Collision|SetCollisionResponsetoChannel (Variables|Default|GetBox) "ECC_Pawn" "ECR_Overlap")
            (Variables|/Game/MarioGameInstance.MarioGameInstance_C|SetMarioWasJustHit (Variables|Default|GetMario%20Game%20Instance) true)
            (Default|InvulnerabilityAnimation (Variables|Default|GetAs%20Mario%20BP))
            (Utilities|FlowControl|Delay 3.0)
            (Variables|/Game/MarioGameInstance.MarioGameInstance_C|SetMarioWasJustHit (Variables|Default|GetMario%20Game%20Instance) false)
            (Collision|SetCollisionResponsetoChannel (Variables|Collision|GetCapsuleComponent) "ECC_Pawn" "ECR_Block")
            (Collision|SetCollisionResponsetoChannel (Variables|Default|GetBrickHitCollision) "ECC_Pawn" "ECR_Overlap")))))))

(event Custom|DeathByFireball/StarMario/Koopa
  (bind _charactermovement (Variables|Character|GetCharacterMovement))
  (bind _capsulecomponent (Variables|Collision|GetCapsuleComponent))
  (bind _capsulecomponent_2 (Variables|Collision|GetCapsuleComponent))
  (bind _returnvalue (Transformation|GetWorldTransform _capsulecomponent))
  (bind _returnvalue_2 (Transformation|GetWorldTransform _capsulecomponent_2))
  ;[1 1 1] Death by fire ball / star mario / koopa logic
  (Utilities|FlowControl|DoOnce false
    (:Completed
      (bind _asmario_game_instance (Utilities|Casting|CastToMarioGameInstance (Game|GetGameInstance)))
      (Default|Add100Points _asmario_game_instance)
      (Components|MoveComponentTo _capsulecomponent (Math|Vector|MakeVector (.x (.location _returnvalue)) (.y (.location _returnvalue)) (+ (.z (.location _returnvalue)) 4e+01)) "180.000000,0.000000, 0" false false 0.01 false)
      (Collision|SetCollisionEnabled (Variables|Character|GetMesh) "NoCollision")
      (Components|Movement|StopMovementImmediately _charactermovement)
      (Pawn|Components|CharacterMovement|DisableMovement _charactermovement)
      (CallFunction|Death)
      (Components|MoveComponentTo _capsulecomponent_2 (Math|Vector|MakeVector (.x (.location _returnvalue_2)) (.y (.location _returnvalue_2)) (- (.z (.location _returnvalue_2)) 2e+02)) (.rotation _returnvalue_2) false false 0.5 false)
      (Actor|DestroyActor))))

(event EventBeginPlay
  (Pawn|SpawnDefaultController)
  (bind _asmario_game_instance (Utilities|Casting|CastToMarioGameInstance (Game|GetGameInstance)))
  (if (Variables|/Game/MarioGameInstance.MarioGameInstance_C|GetEnteredLevel2 _asmario_game_instance)
    (bind _returnvalue (Rendering|Material|CreateDynamicMaterialInstance (Variables|Character|GetMesh) 0 "/Game/Characters/Goomba/Materials/body_a_004Blue.body_a_004Blue" "None" :!class /Script/Engine.PrimitiveComponent))
    (Rendering|Material|SetMaterial (Variables|Character|GetMesh) 0 _returnvalue)
    (bind _returnvalue_2 (Rendering|Material|CreateDynamicMaterialInstance (Variables|Character|GetMesh) 1 "/Game/Characters/Goomba/Materials/body_b_004Blue.body_b_004Blue" "None" :!class /Script/Engine.PrimitiveComponent))
    (Rendering|Material|SetMaterial (Variables|Character|GetMesh) 1 _returnvalue_2)))

(event EventTick
  (params (DeltaSeconds :type Float%20%28single-precision%29))
  (bind _box (Variables|Default|GetBox))
  (Utilities|FlowControl|Sequence
    (:then_0
      (Pawn|Input|AddMovementInput (Variables|Default|GetMovementDirection) 0.4 false))
    (:then_1
      (bind _asmario_game_instance (Utilities|Casting|CastToMarioGameInstance (Game|GetGameInstance)))
      (if (Variables|/Game/MarioGameInstance.MarioGameInstance_C|GetStarMario _asmario_game_instance)
        (Collision|SetCollisionEnabled _box "NoCollision")
        (else
          (Collision|SetCollisionEnabled _box "QueryAndPhysics"))))))

(event Collision|EventActorBeginOverlap
  (params (OtherActor :type Actor%20Object%20Reference))
  (Utilities|Casting|CastToFireBall OtherActor)
  (CallFunction|DeathbyFireball/StarMario/Koopa))

(event Collision|EventHit
  (params (MyComp :type Primitive%20Component%20Object%20Reference) (Other :type Actor%20Object%20Reference) (OtherComp :type Primitive%20Component%20Object%20Reference) (bSelfMoved :type Boolean) (HitLocation :type Vector :default "0, 0, 0") (HitNormal :type Vector :default "0, 0, 0") (NormalImpulse :type Vector :default "0, 0, 0") (Hit :type Hit%20Result%20Structure%20%28by%20ref%29))
  (Utilities|FlowControl|Sequence
    (:then_0
      (if (or (Actor|ActorHasTag Other "Goomba") (Actor|ActorHasTag Other "HitActor"))
        (Utilities|FlowControl|FlipFlop
          (:A
            (Variables|Default|SetMovementDirection "1.000000,0.000000, 0"))
          (:B
            (Variables|Default|SetMovementDirection "-1.000000,0.000000, 0")))))
    (:then_1
      (Utilities|Casting|CastToKoopa_Shell_BP Other)
      (CallFunction|DeathbyFireball/StarMario/Koopa)
      (Audio|PlaySound2D "/Game/Sound_Effects/StompSound.StompSound" 1.0 1.0 0.0 0 0))))

(fn ConstructionScript)

(fn Death
  (Components|Animation|PlayAnimation (Variables|Character|GetMesh) "/Game/Characters/Goomba/Animations/Goomba_Death.Goomba_Death" false))