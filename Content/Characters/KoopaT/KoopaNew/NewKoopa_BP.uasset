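; Koopa enemy character for a Mario-style game that walks along X and reverses when it hits a tagged Koopa, Goomba or HitActor.
; Fireball or shell overlaps kill it, awarding 200 points and dropping a flipped, collisionless shell out of view.
; A stomp event awards 100 points, bounces Mario and leaves a shell, briefly toggling collision before destroying the Koopa.
; Both deaths spawn a hit effect and floating score widget.
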(event Custom|DeathByFireball/StarMario/Koopa
  (bind _returnvalue (Transformation|GetActorLocation))
  ;[1 1 1] Death by fire ball / star mario / koopa shell custom event
  (Utilities|FlowControl|DoOnce false
    (:Completed
      (bind _asmario_game_instance (Utilities|Casting|CastToMarioGameInstance (Game|GetGameInstance)))
      (Game|SpawnActorfromClass "/Game/Characters/Goomba/Niagara/FXVarietyPack/Blueprints/BP_ky_hit2.BP_ky_hit2_C" (Math|Transform|MakeTransform (Math|Vector|MakeVector (.x _returnvalue) (+ (.y _returnvalue) 5e+01) (.z _returnvalue)) "0, 0, 0" "0.600000,0.600000,0.600000") "Undefined" 0 0)
      (Utilities|FlowControl|Sequence
        (:then_0
          (Default|Add200Points _asmario_game_instance)
          (Collision|SetCollisionEnabled (Variables|Collision|GetCapsuleComponent) "NoCollision")
          (Rendering|SetActorHiddenInGame true)
          (bind _returnvalue_2 (Game|SpawnActorfromClass "/Game/Characters/Koopa/Koopa_Shell_BP.Koopa_Shell_BP_C" (Transformation|GetActorTransform) "Undefined" 0 0))
          (bind _output_get (Variables|Default|SetKoopaShellActor _returnvalue_2))
          (bind _output_get_2 (Variables|Default|SetKoopaShellCapsule%20Component (Variables|/Script/Engine.Character|GetCapsuleComponent _output_get)))
          (Collision|SetCollisionEnabled _output_get_2 "NoCollision")
          (Components|MoveComponentTo (Variables|Default|GetKoopaShellCapsule%20Component) (Math|Vector|MakeVector (.x (Variables|/Script/Engine.SceneComponent|GetRelativeLocation _output_get_2)) (.y (Variables|/Script/Engine.SceneComponent|GetRelativeLocation _output_get_2)) (+ (.z (Variables|/Script/Engine.SceneComponent|GetRelativeLocation _output_get_2)) 4e+01)) "0.000000,90.000000,180.000000" false false 0.01 false)
          (Components|MoveComponentTo (Variables|Default|GetKoopaShellCapsule%20Component) (Math|Vector|MakeVector (.x (Variables|/Script/Engine.SceneComponent|GetRelativeLocation (Variables|Default|GetKoopaShellCapsule%20Component))) (.y (Variables|/Script/Engine.SceneComponent|GetRelativeLocation (Variables|Default|GetKoopaShellCapsule%20Component))) (- (.z (Variables|/Script/Engine.SceneComponent|GetRelativeLocation (Variables|Default|GetKoopaShellCapsule%20Component))) 2e+02)) "0.000000,90.000000,180.000000" false false 0.4 false)
          (Actor|DestroyActor))
        (:then_1
          (CallFunction|200PointsText))))))

(event Custom|Death%20by%20stomp
  ;[1 1 1] Death when stomped by mario custom event
  (Variables|Default|SetMarioSteppedOn true)
  (bind _returnvalue (Actor|GetActorOfClass "/Game/Characters/Mario/Mario_BP.Mario_BP_C"))
  (Variables|Default|SetAs%20Mario%20BP _returnvalue)
  (Game|SpawnActorfromClass "/Game/Characters/Goomba/Niagara/FXVarietyPack/Blueprints/BP_ky_hit2.BP_ky_hit2_C" (Math|Transform|MakeTransform (Transformation|GetWorldLocation (Variables|Collision|GetCapsuleComponent)) "0, 0, 0" "0.600000,0.600000,0.600000") "Undefined" 0 0)
  (bind _asmario_game_instance (Utilities|Casting|CastToMarioGameInstance (Game|GetGameInstance)))
  (Utilities|FlowControl|Sequence
    (:then_0
      (CallFunction|100PointsText))
    (:then_1
      (Default|Add100Points _asmario_game_instance)
      (Variables|/Script/Engine.CharacterMovementComponent|SetBrakingDecelerationFalling (Variables|/Script/Engine.Character|GetCharacterMovement (Variables|Default|GetAs%20Mario%20BP)) 1e+08)
      (Audio|PlaySound2D "/Game/Sound_Effects/StompSound.StompSound" 1.0 1.0 0.0 0 0)
      (Character|LaunchCharacter (Variables|Default|GetAs%20Mario%20BP) "0.000000,0.0,300.000000" false true)
      (bind _returnvalue_2 (Game|SpawnActorfromClass "/Game/Characters/Koopa/Koopa_Shell_BP.Koopa_Shell_BP_C" (Math|Transform|MakeTransform (.location (Transformation|GetActorTransform)) "0, 0, 0" "0.800000,0.800000,0.800000") "Undefined" 0 0))
      (Collision|SetCollisionEnabled (Variables|/Script/Engine.Character|GetCapsuleComponent _returnvalue_2) "NoCollision")
      (Utilities|FlowControl|Delay 0.02)
      (Variables|/Script/Engine.CharacterMovementComponent|SetBrakingDecelerationFalling (Variables|/Script/Engine.Character|GetCharacterMovement (Variables|Default|GetAs%20Mario%20BP)) 0.0)
      (Collision|SetCollisionEnabled (Variables|/Script/Engine.Character|GetCapsuleComponent _returnvalue_2) "QueryOnly")
      (Utilities|FlowControl|Delay 0.01)
      (Variables|Default|SetMarioSteppedOn false)
      (Utilities|FlowControl|Delay 0.01)
      (Actor|DestroyActor))))

(event EventBeginPlay
  ;[1 1 1] To be able to move
  (Pawn|SpawnDefaultController))

(event Collision|EventActorBeginOverlap
  (params (OtherActor :type Actor%20Object%20Reference))
  ;[1 1 1] Death by fire ball
  (Utilities|FlowControl|Sequence
    (:then_0
      (Utilities|Casting|CastToFireBallMesh OtherActor)
      (CallFunction|DeathbyFireball/StarMario/Koopa))
    (:then_1
      (if (Variables|Default|GetMarioSteppedOn)
        ;[1 1 1] Death by koopa shell
        (Utilities|FlowControl|Delay 0.1))
      (Utilities|Casting|CastToKoopa_Shell_BP OtherActor)
      (CallFunction|DeathbyFireball/StarMario/Koopa)
      (Utilities|FlowControl|DoOnce false
        (:Completed
          (Audio|PlaySound2D "/Game/Sound_Effects/StompSound.StompSound" 1.0 1.0 0.0 0 0))))))

(event EventTick
  (params (DeltaSeconds :type Float%20%28single-precision%29))
  ;[1 1 1] Initial movement input
  (Utilities|FlowControl|Sequence
    (:then_0
      (Pawn|Input|AddMovementInput (Variables|Default|GetMovementDirection) 0.4 false))))

(event Collision|EventHit
  (params (MyComp :type Primitive%20Component%20Object%20Reference) (Other :type Actor%20Object%20Reference) (OtherComp :type Primitive%20Component%20Object%20Reference) (bSelfMoved :type Boolean) (HitLocation :type Vector :default "0, 0, 0") (HitNormal :type Vector :default "0, 0, 0") (NormalImpulse :type Vector :default "0, 0, 0") (Hit :type Hit%20Result%20Structure%20%28by%20ref%29))
  ;[1 1 1] Change direction when necessary
  (if (Math|Boolean|ORBoolean (Actor|ActorHasTag Other "Koopa") (Actor|ActorHasTag Other "HitActor") (Actor|ActorHasTag Other "Goomba"))
    (Utilities|FlowControl|FlipFlop
      (:A
        (Transformation|SetActorRelativeRotation "0,-90.000000, 0")
        (Variables|Default|SetMovementDirection "1.000000,0.000000, 0"))
      (:B
        (Transformation|SetActorRelativeRotation "0,90.000000, 0")
        (Variables|Default|SetMovementDirection "-1.000000,0.000000, 0")))))

(fn ConstructionScript)

(fn 100PointsText
  (bind _returnvalue (Transformation|GetActorTransform))
  (bind _returnvalue_2 (Game|SpawnActorfromClass "/Game/Characters/PointsText_BP.PointsText_BP_C" (Math|Transform|MakeTransform (Math|Vector|MakeVector (.x (.location _returnvalue)) (+ (.y (.location _returnvalue)) 1e+02) (+ (.z (.location _returnvalue)) 1e+02)) "0,90.000000, 0" "1,1,1") "Undefined" 0 0))
  (bind _returnvalue_3 (UserInterface|CreateWidget "/Game/HUD/Points_Text/100_Points_Widget.100_Points_Widget_C"))
  (UserInterface|SetWidget (Variables|/Game/Characters/PointsText_BP.PointsText_BP_C|GetPoints _returnvalue_2) _returnvalue_3))

(fn 200PointsText
  (bind _returnvalue (Transformation|GetActorTransform))
  (bind _returnvalue_2 (Game|SpawnActorfromClass "/Game/Characters/PointsText_BP.PointsText_BP_C" (Math|Transform|MakeTransform (Math|Vector|MakeVector (.x (.location _returnvalue)) (+ (.y (.location _returnvalue)) 1e+02) (+ (.z (.location _returnvalue)) 1e+02)) "0,90.000000, 0" "1,1,1") "Undefined" 0 0))
  (bind _returnvalue_3 (UserInterface|CreateWidget "/Game/HUD/Points_Text/200_Points_Widget.200_Points_Widget_C"))
  (UserInterface|SetWidget (Variables|/Game/Characters/PointsText_BP.PointsText_BP_C|GetPoints _returnvalue_2) _returnvalue_3))