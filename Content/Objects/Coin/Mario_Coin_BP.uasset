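; Mario_Coin_BP is a collectible coin actor that Mario picks up by overlapping it.
; On capsule overlap with Mario_BP, it tells MarioGameInstance to add a coin and 200 points, then plays a 2D sound and spawns a spark effect at its location.
; It disables capsule collision and hides the mesh immediately, then destroys itself after a short delay.
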(event OnComponentBeginOverlap(CapsuleComponent)
  (params (OverlappedComponent :type Primitive%20Component%20Object%20Reference) (OtherActor :type Actor%20Object%20Reference) (OtherComp :type Primitive%20Component%20Object%20Reference) (OtherBodyIndex :type Integer) (bFromSweep :type Boolean) (SweepResult :type Hit%20Result%20Structure%20%28by%20ref%29))
  (Utilities|Casting|CastToMario_BP OtherActor)
  (bind _asmario_game_instance (Utilities|Casting|CastToMarioGameInstance (Game|GetGameInstance)))
  (Default|AddCoin _asmario_game_instance)
  (Default|Add200Points _asmario_game_instance)
  (Audio|PlaySound2D "/Game/Sound_Effects/CoinSound.CoinSound" 1.0 1.0 0.0 0 0)
  (Niagara|SpawnSystematLocation "/Game/Objects/Coin/Niagara/NE_Sparks_System.NE_Sparks_System" (Transformation|GetActorLocation))
  (Collision|SetCollisionEnabled (Variables|Collision|GetCapsuleComponent) "NoCollision")
  (Development|SetHiddeninGame (Variables|Character|GetMesh) true false)
  (Utilities|FlowControl|Delay 1.0)
  (Actor|DestroyActor))

(event EventBeginPlay)

(event Collision|EventActorBeginOverlap
  (params (OtherActor :type Actor%20Object%20Reference)))

(event EventTick
  (params (DeltaSeconds :type Float%20%28single-precision%29)))

(fn ConstructionScript)