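; Power-up mushroom character for a Mario-style game that emerges on spawn and walks on its own along the X axis.
; BeginPlay spawns a controller and runs a show-up macro that dips the capsule, unhides the mesh and raises it.
; Tick feeds constant movement input, and hits on "HitActor"-tagged actors flip direction and facing.
; Overlapping Mario makes him jump and power up, plays a sound and destroys the mushroom.
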(event OnComponentBeginOverlap(CapsuleComponent)
  (params (OverlappedComponent :type Primitive%20Component%20Object%20Reference) (OtherActor :type Actor%20Object%20Reference) (OtherComp :type Primitive%20Component%20Object%20Reference) (OtherBodyIndex :type Integer) (bFromSweep :type Boolean) (SweepResult :type Hit%20Result%20Structure%20%28by%20ref%29))
  (bind _asmario_bp (Utilities|Casting|CastToMario_BP OtherActor))
  (Character|Jump _asmario_bp)
  (Default|PowerUp _asmario_bp)
  (Audio|PlaySound2D "/Game/Sound_Effects/PowerUpSound.PowerUpSound" 1.0 1.0 0.0 0 0)
  (Actor|DestroyActor))

(event EventBeginPlay
  (Pawn|SpawnDefaultController)
  (Utilities|MushroomShowUp))

(event Collision|EventHit
  (params (MyComp :type Primitive%20Component%20Object%20Reference) (Other :type Actor%20Object%20Reference) (OtherComp :type Primitive%20Component%20Object%20Reference) (bSelfMoved :type Boolean) (HitLocation :type Vector :default "0, 0, 0") (HitNormal :type Vector :default "0, 0, 0") (NormalImpulse :type Vector :default "0, 0, 0") (Hit :type Hit%20Result%20Structure%20%28by%20ref%29))
  (if (Actor|ActorHasTag Other "HitActor")
    (Utilities|FlowControl|FlipFlop
      (:A
        (Transformation|SetActorRelativeRotation "0,-90.000000, 0")
        (Variables|Default|SetMovementDirection "1.000000,0.000000, 0"))
      (:B
        (Transformation|SetActorRelativeRotation "0,90.000000, 0")
        (Variables|Default|SetMovementDirection "-1.000000,0.000000, 0")))))

(event EventTick
  (params (DeltaSeconds :type Float%20%28single-precision%29))
  (Pawn|Input|AddMovementInput (Variables|Default|GetMovementDirection) 0.8 false))

(fn ConstructionScript)