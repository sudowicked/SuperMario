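; Star power-up Character for a Mario game that rises on spawn, then travels horizontally while bouncing.
; Tick drives movement and relaunches it after landing, a looping timer raises gravity while falling, and hits on StarActor-tagged objects flip direction.
; Mario's overlap sets StarMario on the GameInstance, awards points, changes his material and hides the star.
; StarMario clears 10 seconds after overlap ends, before the star is destroyed, or upon level 1 completion.
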(event OnComponentBeginOverlap(CapsuleComponent)
  (params (OverlappedComponent :type Primitive%20Component%20Object%20Reference) (OtherActor :type Actor%20Object%20Reference) (OtherComp :type Primitive%20Component%20Object%20Reference) (OtherBodyIndex :type Integer) (bFromSweep :type Boolean) (SweepResult :type Hit%20Result%20Structure%20%28by%20ref%29))
  ;[1 1 1] Calling the material change custom event from mario bp after overlap
  (bind _asmario_bp (Utilities|Casting|CastToMario_BP OtherActor))
  (Utilities|FlowControl|DoOnce false
    (:Completed
      (Audio|PlaySound2D "/Game/Sound_Effects/PowerUpSound.PowerUpSound" 1.0 1.0 0.0 0 0)
      (bind _asmario_game_instance (Utilities|Casting|CastToMarioGameInstance (Game|GetGameInstance)))
      (Variables|/Game/MarioGameInstance.MarioGameInstance_C|SetStarMario _asmario_game_instance true)
      (Default|Add1000Points _asmario_game_instance)
      (Default|MaterialChange _asmario_bp)
      (Development|SetHiddeninGame (Variables|Character|GetMesh) true false)
      (Collision|SetCollisionResponsetoChannel (Variables|Collision|GetCapsuleComponent) "ECC_GameTraceChannel1" "ECR_Ignore")
      (Pawn|Components|CharacterMovement|DisableMovement (Variables|Character|GetCharacterMovement)))))

(event OnComponentHit(CapsuleComponent)
  (params (HitComponent :type Primitive%20Component%20Object%20Reference) (OtherActor :type Actor%20Object%20Reference) (OtherComp :type Primitive%20Component%20Object%20Reference) (NormalImpulse :type Vector :default "0, 0, 0") (Hit :type Hit%20Result%20Structure%20%28by%20ref%29))
  ;[1 1 1] Direction change after certain object hit
  (if (Actor|ActorHasTag OtherActor "StarActor")
    (Utilities|FlowControl|FlipFlop
      (:A
        (Variables|Default|SetMovementDirection "1.000000, 0, 0"))
      (:B
        (Variables|Default|SetMovementDirection "-1.000000, 0, 0")))))

(event OnComponentEndOverlap(CapsuleComponent)
  (params (OverlappedComponent :type Primitive%20Component%20Object%20Reference) (OtherActor :type Actor%20Object%20Reference) (OtherComp :type Primitive%20Component%20Object%20Reference) (OtherBodyIndex :type Integer))
  ;[1 1 1] Return to mario default state on end overlap after 10 seconds
  (Utilities|Casting|CastToMario_BP OtherActor)
  (Utilities|FlowControl|Delay 1e+01)
  (bind _asmario_game_instance (Utilities|Casting|CastToMarioGameInstance (Game|GetGameInstance)))
  (Variables|/Game/MarioGameInstance.MarioGameInstance_C|SetStarMario _asmario_game_instance false)
  (Utilities|FlowControl|Delay 0.2)
  (Actor|DestroyActor))

(event EventBeginPlay
  ;[1 1 1] Making star moveable and show up animation
  (Pawn|SpawnDefaultController)
  (Utilities|StarShowUp
    (:Completed
      (Utilities|Time|SetTimerbyFunctionName 0 "isFalling" 0.1 true))))

(event EventTick
  (params (DeltaSeconds :type Float%20%28single-precision%29))
  ;[1 1 1] Adding constant bouncy movement
  (Utilities|FlowControl|Sequence
    (:then_0
      (Pawn|Input|AddMovementInput (Variables|Default|GetMovementDirection) 0.5 false)
      (if (Variables|Default|Getlanded)
        (Character|LaunchCharacter "0, 0,1300.000000" false false)
        (Variables|Default|Setlanded false)))
    (:then_1
      ;[1 1 1] Stopping star form if mario touches the flag
      (bind _asmario_game_instance (Utilities|Casting|CastToMarioGameInstance (Game|GetGameInstance)))
      (if (Variables|/Game/MarioGameInstance.MarioGameInstance_C|GetLevel1Complete _asmario_game_instance)
        (Variables|/Game/MarioGameInstance.MarioGameInstance_C|SetStarMario _asmario_game_instance false)))))

(event EventOnLanded
  (params (Hit :type Hit%20Result%20Structure%20%28by%20ref%29))
  ;[1 1 1] Adding constant bouncy movement
  (Variables|Default|Setlanded true))

(fn ConstructionScript)

(fn IsFalling
  (bind _charactermovement (Variables|Character|GetCharacterMovement))
  (if (AI|Components|NavMovement|IsFalling _charactermovement)
    (Variables|/Script/Engine.CharacterMovementComponent|SetGravityScale _charactermovement 3.7)))