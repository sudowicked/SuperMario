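; Plant hazard, apparently a piranha-plant-style enemy, that bobs vertically and kills Mario on contact.
; From BeginPlay, PlantMovement uses eased MoveComponentTo calls to raise and lower the capsule relative to its current location, pausing briefly at the top.
; The event calls itself after each descent to loop indefinitely, with no pause at the bottom.
; Any actor overlap that casts to Mario_BP triggers MarioDeath.
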(event Custom|PlantMovement
  (bind _capsulecomponent (Variables|Collision|GetCapsuleComponent))
  (bind _capsulecomponent_2 (Variables|Collision|GetCapsuleComponent))
  (bind _relativelocation (Variables|/Script/Engine.SceneComponent|GetRelativeLocation _capsulecomponent))
  (bind _relativelocation_2 (Variables|/Script/Engine.SceneComponent|GetRelativeLocation _capsulecomponent_2))
  (Components|MoveComponentTo _capsulecomponent_2 (Math|Vector|MakeVector (.x _relativelocation_2) (.y _relativelocation_2) (+ (.z _relativelocation_2) 2e+02)) "0, 0, 0" true true 2.5 false)
  (Utilities|FlowControl|Delay 0.5)
  (Components|MoveComponentTo _capsulecomponent (Math|Vector|MakeVector (.x _relativelocation) (.y _relativelocation) (+ (.z _relativelocation) -2e+02)) "0, 0, 0" true true 2.5 false)
  (CallFunction|PlantMovement))

(event EventBeginPlay
  (CallFunction|PlantMovement))

(event Collision|EventActorBeginOverlap
  (params (OtherActor :type Actor%20Object%20Reference))
  (bind _asmario_bp (Utilities|Casting|CastToMario_BP OtherActor))
  (Default|MarioDeath _asmario_bp))

(fn ConstructionScript)