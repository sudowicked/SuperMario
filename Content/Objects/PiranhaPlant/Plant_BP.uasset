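; Piranha plant enemy that rises and sinks in a repeating MoveComponentTo cycle and hurts Mario on contact.
; A detection volume holds it while Mario is near, with Tick using a DoOnce to restart the cycle from the starting position.
; Contact kills or powers down Mario, with brief invulnerability, while Star Mario or a fireball triggers the plant's death and points popup.
; Game instance level-exit flags destroy or pause it on BeginPlay.
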(event OnComponentBeginOverlap(CapsuleComponent)
  (params (OverlappedComponent :type Primitive%20Component%20Object%20Reference) (OtherActor :type Actor%20Object%20Reference) (OtherComp :type Primitive%20Component%20Object%20Reference) (OtherBodyIndex :type Integer) (bFromSweep :type Boolean) (SweepResult :type Hit%20Result%20Structure%20%28by%20ref%29))
  ;[1 1 1] Mario kill if mario steps on plant/plant kill if mario in star form
  (bind _asmario_bp (Utilities|Casting|CastToMario_BP OtherActor))
  (Variables|Default|SetAs%20Mario%20BP _asmario_bp)
  (bind _asmario_game_instance (Utilities|Casting|CastToMarioGameInstance (Game|GetGameInstance)))
  (bind _output_get (Variables|Default|SetMario%20Game%20Instance _asmario_game_instance))
  (if (not (Variables|/Game/MarioGameInstance.MarioGameInstance_C|GetMarioWasJustHit _asmario_game_instance))
    (if (Variables|/Game/MarioGameInstance.MarioGameInstance_C|GetStarMario _asmario_game_instance)
      (CallFunction|PlantDeath)
      (Default|Add200Points _asmario_game_instance)
      (Audio|PlaySound2D "/Game/Sound_Effects/StompSound.StompSound" 1.0 1.0 0.0 0 0)
      (elif (== (Variables|/Game/MarioGameInstance.MarioGameInstance_C|GetMarioState _output_get) 0)
        (Default|MarioDeath (Variables|Default|GetAs%20Mario%20BP))
        (elif (== (Variables|/Game/MarioGameInstance.MarioGameInstance_C|GetMarioState _output_get) 1)
          (Default|PowerDown (Variables|Default|GetAs%20Mario%20BP))
          (Audio|PlaySound2D "/Game/Sound_Effects/PipeEnterExit.PipeEnterExit" 1.0 1.0 0.0 0 0)
          (Collision|SetCollisionResponsetoChannel (Variables|/Script/Engine.Character|GetCapsuleComponent (Variables|Default|GetAs%20Mario%20BP)) "ECC_Pawn" "ECR_Ignore")
          (Variables|/Game/MarioGameInstance.MarioGameInstance_C|SetMarioWasJustHit (Variables|Default|GetMario%20Game%20Instance) true)
          (Default|InvulnerabilityAnimation (Variables|Default|GetAs%20Mario%20BP))
          (Utilities|FlowControl|Delay 3.0)
          (Variables|/Game/MarioGameInstance.MarioGameInstance_C|SetMarioWasJustHit (Variables|Default|GetMario%20Game%20Instance) false)
          (Collision|SetCollisionResponsetoChannel (Variables|Collision|GetCapsuleComponent) "ECC_Pawn" "ECR_Overlap")
          (else
            (Default|CookPowerDowntoMario (Variables|Default|GetAs%20Mario%20BP))
            (Audio|PlaySound2D "/Game/Sound_Effects/PipeEnterExit.PipeEnterExit" 1.0 1.0 0.0 0 0)
            (Collision|SetCollisionResponsetoChannel (Variables|Collision|GetCapsuleComponent) "ECC_Pawn" "ECR_Ignore")
            (Variables|/Game/MarioGameInstance.MarioGameInstance_C|SetMarioWasJustHit (Variables|Default|GetMario%20Game%20Instance) true)
            (Default|InvulnerabilityAnimation (Variables|Default|GetAs%20Mario%20BP))
            (Utilities|FlowControl|Delay 3.0)
            (Variables|/Game/MarioGameInstance.MarioGameInstance_C|SetMarioWasJustHit (Variables|Default|GetMario%20Game%20Instance) false)
            (Collision|SetCollisionResponsetoChannel (Variables|Collision|GetCapsuleComponent) "ECC_Pawn" "ECR_Overlap")))))))

(event OnComponentBeginOverlap(MarioDetectionCollision)
  (params (OverlappedComponent :type Primitive%20Component%20Object%20Reference) (OtherActor :type Actor%20Object%20Reference) (OtherComp :type Primitive%20Component%20Object%20Reference) (OtherBodyIndex :type Integer) (bFromSweep :type Boolean) (SweepResult :type Hit%20Result%20Structure%20%28by%20ref%29))
  ;[1 1 1] Deciding whether the plant can move or not
  (Utilities|Casting|CastToMario_BP OtherActor)
  (Variables|Default|SetPlantCantMove true))

(event OnComponentEndOverlap(MarioDetectionCollision)
  (params (OverlappedComponent :type Primitive%20Component%20Object%20Reference) (OtherActor :type Actor%20Object%20Reference) (OtherComp :type Primitive%20Component%20Object%20Reference) (OtherBodyIndex :type Integer))
  ;[1 1 1] Deciding whether the plant can move or not
  (Utilities|Casting|CastToMario_BP OtherActor)
  (Variables|Default|SetPlantCantMove false))

(event Custom|PlantMovement
  (bind _capsulecomponent (Variables|Collision|GetCapsuleComponent))
  (bind _capsulecomponent_2 (Variables|Collision|GetCapsuleComponent))
  (bind _relativelocation (Variables|/Script/Engine.SceneComponent|GetRelativeLocation _capsulecomponent))
  (bind _relativelocation_2 (Variables|/Script/Engine.SceneComponent|GetRelativeLocation _capsulecomponent_2))
  ;[1 1 1] Custom event for the up and down plant movement
  (if (not (Variables|Default|GetPlantCantMove))
    (Variables|Default|SetPlantInStartingPosition false)
    (Components|MoveComponentTo _capsulecomponent_2 (Math|Vector|MakeVector (.x _relativelocation_2) (.y _relativelocation_2) (+ (.z _relativelocation_2) 195.0)) "0, 0, 0" true true 2.0 false)
    (Utilities|FlowControl|Delay 0.3)
    (Components|MoveComponentTo _capsulecomponent (Math|Vector|MakeVector (.x _relativelocation) (.y _relativelocation) (+ (.z _relativelocation) -195.0)) "0, 0, 0" true true 2.0 false)
    (Variables|Default|SetPlantInStartingPosition true)
    (CallFunction|PlantMovement)))

(event Custom|Plant_Death
  (bind _capsulecomponent (Variables|Collision|GetCapsuleComponent))
  (bind _relativelocation (Variables|/Script/Engine.SceneComponent|GetRelativeLocation _capsulecomponent))
  ;[1 1 1] Plant death custom event
  (CallFunction|200PointsText)
  (Components|Animation|PlayAnimation (Variables|Character|GetMesh) "/Game/Objects/PiranhaPlant/Plant_Death.Plant_Death" false)
  (Collision|SetActorEnableCollision false)
  (Components|MoveComponentTo _capsulecomponent (Math|Vector|MakeVector (.x _relativelocation) (.y _relativelocation) (- (.z _relativelocation) 2e+02)) "0, 0, 0" false false 0.4 false)
  (Actor|DestroyActor))

(event Collision|EventActorBeginOverlap
  (params (OtherActor :type Actor%20Object%20Reference))
  ;[1 1 1] Plant death when hit by fireball
  (Utilities|Casting|CastToFireBallMesh OtherActor)
  (CallFunction|PlantDeath))

(event EventTick
  (params (DeltaSeconds :type Float%20%28single-precision%29))
  (bind _plantinstartingposition (Variables|Default|GetPlantInStartingPosition))
  (if (Variables|Default|GetPlantCantMove)
    (if _plantinstartingposition
      (goto _label Reset))
    (elif _plantinstartingposition
      (Utilities|FlowControl|DoOnce false :!label _label
        (:Completed
          (CallFunction|PlantMovement))))))

(event EventBeginPlay
  (bind _capsulecomponent (Variables|Collision|GetCapsuleComponent))
  ;[1 1 1] List of options on begin play
  (bind _asmario_game_instance (Utilities|Casting|CastToMarioGameInstance (Game|GetGameInstance)))
  (if (Variables|/Game/MarioGameInstance.MarioGameInstance_C|GetExitLevel2Pipe _asmario_game_instance)
    (Actor|DestroyActor)
    (elif (Variables|/Game/MarioGameInstance.MarioGameInstance_C|GetExitLevel2 _asmario_game_instance)
      (Variables|Default|SetPlantCantMove true)
      (Collision|SetCollisionEnabled _capsulecomponent "NoCollision")
      (Utilities|FlowControl|Delay 1.5)
      (Collision|SetCollisionEnabled _capsulecomponent "QueryAndPhysics")
      (Variables|Default|SetTags (Variables|Default|GetTag))
      (else
        (Variables|Default|SetTags (Variables|Default|GetTag))))))

(fn ConstructionScript)

(fn 200PointsText
  (bind _returnvalue (Transformation|GetActorTransform))
  (bind _returnvalue_2 (Game|SpawnActorfromClass "/Game/Characters/PointsText_BP.PointsText_BP_C" (Math|Transform|MakeTransform (Math|Vector|MakeVector (.x (.location _returnvalue)) (+ (.y (.location _returnvalue)) 1e+02) (+ (.z (.location _returnvalue)) 1e+02)) "0,90.000000, 0" "1,1,1") "Undefined" 0 0))
  (bind _returnvalue_3 (UserInterface|CreateWidget "/Game/HUD/Points_Text/200_Points_Widget.200_Points_Widget_C"))
  (UserInterface|SetWidget (Variables|/Game/Characters/PointsText_BP.PointsText_BP_C|GetPoints _returnvalue_2) _returnvalue_3))