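; Fire flower power-up Blueprint that rises into view when spawned and is collected when Mario touches it.
; On BeginPlay, Flower Show Up quickly lowers the capsule, unhides the flower, then slowly raises it using chained MoveComponentTo calls.
; Capsule overlap with Mario_BP calls CookMario, adds 1000 points through MarioGameInstance, plays the power-up sound and destroys the actor.
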(event OnComponentBeginOverlap(CapsuleComponent)
  (params (OverlappedComponent :type Primitive%20Component%20Object%20Reference) (OtherActor :type Actor%20Object%20Reference) (OtherComp :type Primitive%20Component%20Object%20Reference) (OtherBodyIndex :type Integer) (bFromSweep :type Boolean) (SweepResult :type Hit%20Result%20Structure%20%28by%20ref%29))
  (bind _asmario_bp (Utilities|Casting|CastToMario_BP OtherActor))
  (Default|CookMario _asmario_bp)
  (bind _asmario_game_instance (Utilities|Casting|CastToMarioGameInstance (Game|GetGameInstance)))
  (Default|Add1000Points _asmario_game_instance)
  (Audio|PlaySound2D "/Game/Sound_Effects/PowerUpSound.PowerUpSound" 1.0 1.0 0.0 0 0)
  (Actor|DestroyActor))

(event EventBeginPlay
  (Utilities|FlowerShowUp))

(event Collision|EventActorBeginOverlap
  (params (OtherActor :type Actor%20Object%20Reference)))

(event EventTick
  (params (DeltaSeconds :type Float%20%28single-precision%29)))

(fn ConstructionScript)