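; FireBall_BP is a bouncing fireball Character that travels along its MovementDirection.
; On BeginPlay it spawns its default controller, and Tick applies constant movement input in that direction.
; OnLanded sets a flag that makes the next Tick launch it upward, producing repeated bounces.
; A looping timer raises gravity scale whenever it is falling, with no reset in this graph.
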(event EventBeginPlay
  (Utilities|Time|SetTimerbyFunctionName 0 "isFalling" 0.1 true)
  (Pawn|SpawnDefaultController))

(event EventTick
  (params (DeltaSeconds :type Float%20%28single-precision%29))
  (Utilities|FlowControl|Sequence
    (:then_0
      (Pawn|Input|AddMovementInput (Variables|Default|GetMovement%20Direction) 2.0 false)
      (if (Variables|Default|Getlanded)
        (Character|LaunchCharacter "0, 0,1300.000000" false false)
        (Variables|Default|Setlanded false)))))

(event EventOnLanded
  (params (Hit :type Hit%20Result%20Structure%20%28by%20ref%29))
  (Variables|Default|Setlanded true))

(fn ConstructionScript)

(fn IsFalling
  (bind _charactermovement (Variables|Character|GetCharacterMovement))
  (if (AI|Components|NavMovement|IsFalling _charactermovement)
    (Variables|/Script/Engine.CharacterMovementComponent|SetGravityScale _charactermovement 8.0)))