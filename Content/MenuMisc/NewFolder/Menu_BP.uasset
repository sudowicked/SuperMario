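; Menu page actor for a Mario game that hosts a Menu_Widget and moves the camera between linked menu pages.
; A widget-triggered event picks a page from LinkedMenus by index and blends the player's view target to it.
; Actor collision gates mouse interaction, re-enabling on the target after a delay that is longer during game initialization.
; Tick polls the game instance to disable that interaction once Play is pressed.
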(event Custom|TransitionTo
  (params (NewMenu :type Menu%20BP%20Object%20Reference))
  ;[1 1 1] Camera transition to the desired menu page from the linked menus array
  (Variables|Menu_BP_C|SetNew%20Menu NewMenu NewMenu)
  (Collision|SetActorEnableCollision false)
  (Game|Player|SetViewTargetwithBlend (Game|GetPlayerController 0) NewMenu 3.0 "VTBlend_Cubic" 0.0 false)
  (if (Variables|/Game/MarioGameInstance.MarioGameInstance_C|GetGameInit (Variables|Default|GetAs%20Mario%20Game%20Instance))
    (Utilities|FlowControl|Delay 8.7)
    (Collision|SetActorEnableCollision NewMenu true)
    (Variables|/Game/MarioGameInstance.MarioGameInstance_C|SetGameInit (Variables|Default|GetAs%20Mario%20Game%20Instance) false)
    (else
      (Utilities|FlowControl|Delay 3.0)
      (Collision|SetActorEnableCollision NewMenu true))))

(event Custom|OnTransitionBetweenMenus
  (params (MenuIndex :type Integer))
  ;[1 1 1] Binding "OnTransitionBetweenMenus" custom event to Menu_Widget's "TransitionToLinkedMenu" function so it calls it whenever a button is clicked
  (if (Utilities|Array|IsValidIndex (Variables|Default|GetLinkedMenus))
    (CallFunction|Transitionto (Utilities|Array|Get(acopy) (Variables|Default|GetLinkedMenus) MenuIndex))))

(event EventBeginPlay
  ;[1 1 1] Binding "OnTransitionBetweenMenus" custom event to Menu_Widget's "TransitionToLinkedMenu" function so it calls it whenever a button is clicked
  (bind _asmario_game_instance (Utilities|Casting|CastToMarioGameInstance (Game|GetGameInstance)))
  (Variables|Default|SetAs%20Mario%20Game%20Instance _asmario_game_instance)
  (bind _asmenu_widget (Utilities|Casting|CastToMenu_Widget (UserInterface|GetUserWidgetObject (Variables|Default|GetWidget))))
  (EventDispatchers|BindEventtoTransitiontoLinkedMenu _asmenu_widget (delegate Custom|OnTransitionBetweenMenus))
  (Collision|SetActorEnableCollision false))

(event EventTick
  (params (DeltaSeconds :type Float%20%28single-precision%29))
  ;[1 1 1] Disabling mouse interaction with menu when "Play" is clicked
  (Utilities|IsValid (Variables|Default|GetNew%20Menu)
    (:Is%20Valid
      (bind _asmario_game_instance (Utilities|Casting|CastToMarioGameInstance (Game|GetGameInstance)))
      (if (Variables|/Game/MarioGameInstance.MarioGameInstance_C|GetMainMenuPlayIsPressed _asmario_game_instance)
        (Utilities|FlowControl|DoOnce false
          (:Completed
            (Collision|SetActorEnableCollision (stale Custom|TransitionTo NewMenu) false)))))))

(fn ConstructionScript)